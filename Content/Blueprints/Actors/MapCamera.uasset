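; MapCamera is a possessable map-view pawn from which a player asks to join a match.
; On BeginPlay it moves to the transform of the first PlayerStart found, and on possession it registers itself as MapCamera on the GLOOM player state.
; Pressing PrimeAttack calls AskGameToJoinMatch on the GLOOM controller.
; Direct class spawn, game mode join and team menu calls remain as unconnected nodes.
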(event EventBeginPlay
  (bind _outactors (Actor|GetAllActorsOfClass "/Script/Engine.PlayerStart"))
  (Transformation|SetActorTransform (Transformation|GetActorTransform (Utilities|Array|Get(acopy) _outactors))))

(event EventPossessed
  (params (NewController :type Controller%20Object%20Reference))
  (bind _asgloom_player_state (Utilities|Casting|CastToGLOOM_PlayerState (Variables|/Script/Engine.Controller|GetPlayerState NewController)))
  (Variables|/Game/System/GLOOM_PlayerState.GLOOM_PlayerState_C|SetMapCamera _asgloom_player_state self))

(event Input|ActionEvents|InputActionPrimeAttack
  (params (Key :type Key%20Structure))
  (:Pressed
    (bind _asgloom_controller (Utilities|Casting|CastToGLOOM_Controller (Pawn|GetController)))
    (Default|AskGametoJoinMatch _asgloom_controller)))

(fn ConstructionScript)