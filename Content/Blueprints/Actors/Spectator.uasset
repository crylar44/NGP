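; Spectator pawn for GLOOM that lets a player fly around and open the team menu.
; On BeginPlay it caches the first player controller's GLOOM player state.
; A BecomeOffisialSpectator event sets the floating pawn movement's max speed, and the Menu input asks the GLOOM HUD to show the team menu.
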(event Custom|BecomeOffisialSpectator
  (bind _asfloating_pawn_movement (Utilities|Casting|CastToFloatingPawnMovement (Variables|Default|GetMovementComponent)))
  (Variables|/Script/Engine.FloatingPawnMovement|SetMaxSpeed _asfloating_pawn_movement 1.2e+03))

(event EventBeginPlay
  (bind _asgloom_player_state (Utilities|Casting|CastToGLOOM_PlayerState (Variables|/Script/Engine.Controller|GetPlayerState (Game|GetPlayerController 0))))
  (Variables|Default|SetGLOOM_PlayerState _asgloom_player_state))

(event Input|ActionEvents|InputActionMenu
  (params (Key :type Key%20Structure))
  (:Pressed
    (bind _asgloom_hud (Utilities|Casting|CastToGLOOM_HUD (HUD|GetHUD (Game|GetPlayerController 0))))
    (Default|ShowTeamMenu _asgloom_hud)))

(fn ConstructionScript)