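; Alien Breeder character, the alien class that places and removes alien structures.
; On possession it builds the structure menu, which secondary attack toggles and death removes, and while the menu is active Tick previews the selected structure's placement.
; The Z key line-traces from the camera to remove a targeted alien structure.
; Sphere overlaps start and stop HUD stat tracking for nearby alien structures.
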(event OnComponentBeginOverlap(Sphere)
  (params (OverlappedComponent :type Primitive%20Component%20Object%20Reference) (OtherActor :type Actor%20Object%20Reference) (OtherComp :type Primitive%20Component%20Object%20Reference) (OtherBodyIndex :type Integer) (bFromSweep :type Boolean) (SweepResult :type Hit%20Result%20Structure%20%28by%20ref%29))
  (bind _asstructure_alien (Utilities|Casting|CastToStructure_Alien OtherActor))
  (Default|TrackActorStats (Variables|/Game/System/GLOOM_Controller.GLOOM_Controller_C|GetGloomHUD (Variables|Default|GetGloomController)) _asstructure_alien))

(event OnComponentEndOverlap(Sphere)
  (params (OverlappedComponent :type Primitive%20Component%20Object%20Reference) (OtherActor :type Actor%20Object%20Reference) (OtherComp :type Primitive%20Component%20Object%20Reference) (OtherBodyIndex :type Integer))
  (bind _asstructure_alien (Utilities|Casting|CastToStructure_Alien OtherActor))
  (Default|StopTrackingActorStats (Variables|/Game/System/GLOOM_Controller.GLOOM_Controller_C|GetGloomHUD (Variables|Default|GetGloomController)) _asstructure_alien))

(event EventPossessed
  (params (NewController :type Controller%20Object%20Reference))
  (|CallParentFunction NewController)
  (CallFunction|GetStructureListandMakeWidget))

(event EventTick
  (params (DeltaSeconds :type Float%20%28single-precision%29))
  (|CallParentFunction DeltaSeconds)
  (if (Variables|Default|GetUsingStructureMenu)
    (CallFunction|TickShowSelectedStructurePlacement)))

(event EventDie
  (params (Attacker :type GLOOM%20Controller%20Object%20Reference))
  (|CallParentFunction Attacker)
  (bind _classhud (Variables|Default|GetClassHUD)
    (:then
      (Default|RemoveStructureMenu _classhud))
    (:else)))

(event Input|ActionEvents|InputActionSecondAttack
  (params (Key :type Key%20Structure))
  (:Pressed
    (bind _output_get (Variables|Default|SetUsingStructureMenu (not (Variables|Default|GetUsingStructureMenu))))
    (Default|SetStructureMenuVisibility (Variables|Default|GetClassHUD) _output_get)))

(event Input|KeyboardEvents|Z
  (params (Key :type Key%20Structure))
  (bind _camera (Variables|Default|GetCamera))
  (bind _returnvalue (Transformation|GetWorldLocation _camera))
  (:Pressed
    (bind _outhit (Collision|LineTraceForObjects _returnvalue (+ _returnvalue (* (Math|Vector|GetForwardVector _camera) 1.5e+03)) (Utilities|Array|MakeArray "ObjectTypeQuery1" "ObjectTypeQuery2" "ObjectTypeQuery4") false 0 "ForDuration"))
    (bind _asstructure_alien (Utilities|Casting|CastToStructure_Alien (.HitActor (Collision|BreakHitResult _outhit))))
    (Default|RemoveStructure _asstructure_alien)))

(fn ConstructionScript
  (|CallParentFunction))