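; Alien Drone character Blueprint that gives a short boosted-jump window after each landing.
; On landing it calls the parent handler, then raises the movement component's jump velocity to 1.5 times the class data's jump power.
; A brief Delay then restores the normal jump power, so only jumps made right after touchdown get the boost.
; The construction script only calls its parent.
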(event EventOnLanded
  (params (Hit :type Hit%20Result%20Structure%20%28by%20ref%29))
  (|CallParentFunction Hit)
  (Variables|/Script/Engine.CharacterMovementComponent|SetJumpZVelocity (Variables|Character|GetCharacterMovement) (* (.JumpPower (Utilities|Struct|BreakClassData (Variables|Default|GetClassData))) 1.5))
  (Utilities|FlowControl|Delay 0.2)
  (Variables|/Script/Engine.CharacterMovementComponent|SetJumpZVelocity (Variables|Character|GetCharacterMovement) (.JumpPower (Utilities|Struct|BreakClassData (Variables|Default|GetClassData)))))

(fn ConstructionScript
  (|CallParentFunction))