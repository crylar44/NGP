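; Playable alien Guardian character that turns invisible while standing still and can swallow C4 to become a living bomb.
; Tick watches movement, weapon state, priming and mouth use, starting a timeline before setting the post-process invisibility parameter.
; SecondAttack sphere-traces ahead, briefly locking input on C4 or humans; eaten C4 triggers a delayed explosion.
; It also handles movement and look input, flight-mode switching, and a four-spore cap that destroys the oldest.
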(event Custom|CheckUpOnSpores
  (params (NewSpore :type Actor%20Object%20Reference))
  (bind _activespores (Variables|Default|GetActiveSpores))
  (Utilities|FlowControl|Sequence
    (:then_0
      (if (== (Utilities|Array|Length (Variables|Default|GetActiveSpores)) 4)
        (Actor|DestroyActor (Utilities|Array|Get(acopy) _activespores))
        (Utilities|Array|RemoveIndex _activespores)))
    (:then_1
      (Utilities|Array|Add (Variables|Default|GetActiveSpores) NewSpore))))

(event Custom|SetInvisibility
  (params (Invisible :type Boolean))
  (bind _output_get (Variables|Default|SetInvisible Invisible))
  (Rendering|Material|SetScalarParameterValue (Variables|Default|GetPostProcessDynamicMaterial) "Invisible" (Math|Conversions|ToFloat(Boolean) _output_get) :!class /Script/Engine.MaterialInstanceDynamic))

(event EventTick
  (params (DeltaSeconds :type Float%20%28single-precision%29))
  (bind _usingmouth (Variables|Default|GetUsingMouth))
  (bind _primed (Variables|Default|GetPrimed))
  (bind _charactermovement (Variables|Character|GetCharacterMovement))
  (bind _equipedweapon (Variables|Default|GetEquipedWeapon))
  (bind _returnvalue (not _primed))
  (bind _returnvalue_2 (not _usingmouth))
  (bind _velocity (Variables|/Script/Engine.MovementComponent|GetVelocity _charactermovement))
  (bind _weaponstate (Variables|/Game/Blueprints/Weapons/Weapon.Weapon_C|GetWeaponState _equipedweapon))
  (bind _returnvalue_3 (Math|Vector|VectorLength _velocity))
  (bind _returnvalue_4 (Utilities|Enum|Equal(Enum) _weaponstate "NewEnumerator2"))
  (bind _returnvalue_5 (== _returnvalue_3 0.0))
  (bind _returnvalue_6 (Math|Boolean|ANDBoolean _returnvalue _returnvalue_4 _returnvalue_5 _returnvalue_2))
  (|CallParentFunction DeltaSeconds)
  (if (Math|Boolean|NotEqual(Boolean) (Variables|Default|GetStill) _returnvalue_6)
    (bind _output_get (Variables|Default|SetStill _returnvalue_6))
    (if _output_get
      (Timeline|TimeToChekStillForInvisibility PlayFromStart
        (:Finished
          (CallFunction|SetInvisibility (Variables|Default|GetStill))))
      (else
        (CallFunction|SetInvisibility false)))))

(event Input|ActionEvents|InputActionSecondAttack
  (params (Key :type Key%20Structure))
  (bind _camera (Variables|Default|GetCamera))
  (bind _returnvalue (Transformation|GetWorldLocation _camera))
  (:Pressed
    (bind (_outhit _returnvalue_2) (Collision|SphereTraceForObjects _returnvalue (+ _returnvalue (* (Math|Vector|GetForwardVector _camera) 1.2e+02)) 4e+01 (Utilities|Array|MakeArray "ObjectTypeQuery2") false 0 "None"))
    (if _returnvalue_2
      (bind _asc4 (Utilities|Casting|CastToC4 (.HitActor (Collision|BreakHitResult _outhit)))
        (:then
          (Variables|Default|SetUsingMouth true)
          (Utilities|FlowControl|Delay 0.5)
          (Variables|Default|SetUsingMouth false)
          (Actor|DestroyActor _asc4)
          (Variables|Default|SetPrimed true)
          (CallFunction|SetInvisibility false)
          (Utilities|FlowControl|Delay 1e+01)
          (Game|SpawnActorfromClass "/Game/Blueprints/Events/Explosion.Explosion_C" (Math|Transform|MakeTransform (Transformation|GetActorLocation) "0, 0, 0" "1,1,1") "Undefined" 0 1.5e+03 1e+03 (Variables|Default|GetGloomController) true true "NewEnumerator1" 0))
        (:CastFailed
          (Utilities|Casting|CastToCharacter_Human (.HitActor (Collision|BreakHitResult _outhit)))
          (Variables|Default|SetUsingMouth true)
          (Utilities|FlowControl|Delay 0.8)
          (Variables|Default|SetUsingMouth false))))))

(event Input|AxisEvents|InputAxisLookUp
  (params (AxisValue :type Float%20%28single-precision%29))
  (bind _scenehead (Variables|Default|GetSceneHead))
  (if (Math|Boolean|ANDBoolean (not (Variables|Default|GetDead)) (not (Variables|Default|GetSticky)) (not (Variables|Default|GetUsingMouth)))
    (Transformation|SetRelativeRotation _scenehead (Math|Rotator|MakeRotator 0.0 (Math|Float|Clamp(Float) (+ (.pitch (Variables|/Script/Engine.SceneComponent|GetRelativeRotation _scenehead)) (* AxisValue (Variables|Default|GetLookSensitivity))) -89.0 89.0) 0.0) false false)
    (Default|UpdateFloatingHUDElements (Variables|/Game/System/GLOOM_Controller.GLOOM_Controller_C|GetGloomHUD (Variables|Default|GetGloomController)))))

(event Input|AxisEvents|InputAxisLookRight
  (params (AxisValue :type Float%20%28single-precision%29))
  (if (and (not (Variables|Default|GetDead)) (not (Variables|Default|GetUsingMouth)))
    (Pawn|Input|AddControllerYawInput (* AxisValue (Variables|Default|GetLookSensitivity) 0.5))
    (Default|UpdateFloatingHUDElements (Variables|/Game/System/GLOOM_Controller.GLOOM_Controller_C|GetGloomHUD (Variables|Default|GetGloomController)))))

(event Input|AxisEvents|InputAxisMoveForward
  (params (AxisValue :type Float%20%28single-precision%29))
  (if (Math|Boolean|ANDBoolean (not (Variables|Default|GetDead)) (not (Variables|Default|GetSticky)) (not (Variables|Default|GetUsingMouth)))
    (Class|PawnMovementComponent|AddInputVector (Variables|Character|GetCharacterMovement) (* (select (Utilities|Enum|Equal(Enum) (Variables|/Script/Engine.CharacterMovementComponent|GetMovementMode (Variables|Character|GetCharacterMovement)) "MOVE_Flying") (Math|Vector|GetForwardVector (Variables|Default|GetCamera)) (Transformation|GetActorForwardVector)) AxisValue) false)))

(event Input|AxisEvents|InputAxisMoveRight
  (params (AxisValue :type Float%20%28single-precision%29))
  (if (Math|Boolean|ANDBoolean (not (Variables|Default|GetDead)) (not (Variables|Default|GetSticky)) (not (Variables|Default|GetUsingMouth)))
    (Class|PawnMovementComponent|AddInputVector (Variables|Character|GetCharacterMovement) (* (Transformation|GetActorRightVector) AxisValue) false)))

(fn ConstructionScript
  (|CallParentFunction))

(fn SetFlying
  (params (Flying :type Boolean))
  (bind _output_get (Variables|Default|SetInvisible Flying))
  (if _output_get
    (Variables|Default|SetJumping false)
    (Variables|/Script/Engine.CharacterMovementComponent|SetGravityScale (Variables|Character|GetCharacterMovement) 0.0)
    (Pawn|Components|CharacterMovement|SetMovementMode (Variables|Character|GetCharacterMovement) "MOVE_Flying" 0)
    (else
      (Variables|/Script/Engine.CharacterMovementComponent|SetGravityScale (Variables|Character|GetCharacterMovement) (Variables|Default|GetNormalGravityScale))
      (Pawn|Components|CharacterMovement|SetMovementMode (Variables|Character|GetCharacterMovement) "MOVE_Falling" 0))))