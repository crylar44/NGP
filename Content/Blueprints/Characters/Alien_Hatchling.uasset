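; Playable Alien Hatchling character for GLOOM, a small melee alien that pounces and clings to walls.
; Prime attack launches it along the camera view with some upward bias, and colliding with enemy characters or non-spawner structures deals damage.
; Hitting a steep surface head-on while holding Jump zeroes gravity and velocity to stick, until Jump release, attack or damage.
; A RotationPoint parents the head, but its wall-alignment code never runs.
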(event Collision|EventHit
  (params (MyComp :type Primitive%20Component%20Object%20Reference) (Other :type Actor%20Object%20Reference) (OtherComp :type Primitive%20Component%20Object%20Reference) (bSelfMoved :type Boolean) (HitLocation :type Vector :default "0, 0, 0") (HitNormal :type Vector :default "0, 0, 0") (NormalImpulse :type Vector :default "0, 0, 0") (Hit :type Hit%20Result%20Structure%20%28by%20ref%29))
  (bind _asgloom_character (Utilities|Casting|CastToGLOOM_Character Other)
    (:then
      (if (Utilities|Enum|NotEqual(Enum) (Utilities|Struct|BreakClassData (Variables|Default|GetClassData)) (Utilities|Struct|BreakClassData (Variables|/Game/Blueprints/Characters/GLOOM_Character.GLOOM_Character_C|GetClassData _asgloom_character)))
        (Default|TakeDamage _asgloom_character 8e+01 "0, 0, 0" (Variables|Default|GetGloomController) "NewEnumerator4")))
    (:CastFailed
      (bind _asgloom_structure (Utilities|Casting|CastToGLOOM_Structure Other)
        (:then
          (if (and (Utilities|Enum|NotEqual(Enum) (Utilities|Struct|BreakClassData (Variables|Default|GetClassData)) (.Team (Utilities|Struct|BreakStructureData (Variables|/Game/Blueprints/Structures/GLOOM_Structure.GLOOM_Structure_C|GetStructureData _asgloom_structure)))) (not (.Spawner (Utilities|Struct|BreakStructureData (Variables|/Game/Blueprints/Structures/GLOOM_Structure.GLOOM_Structure_C|GetStructureData _asgloom_structure)))))
            (Default|TakeDamage _asgloom_structure 8e+01 (Variables|Default|GetGloomController))))
        (:CastFailed
          (if (Math|Boolean|ANDBoolean (<= (Math|Vector|DotProduct HitNormal "0, 0,1.000000") 0.5) (<= (Math|Vector|DotProduct HitNormal (Variables|Default|GetLastMoveNormal)) -0.5) (Variables|Default|GetHoldingJump) (not (Variables|Default|GetStickingToWall)))
            (CallFunction|SetStickingtoWall true HitNormal)
            (else
              (|CallParentFunction MyComp Other OtherComp bSelfMoved HitLocation HitNormal NormalImpulse Hit))))))))

(event EventTick
  (params (DeltaSeconds :type Float%20%28single-precision%29))
  (|CallParentFunction DeltaSeconds)
  (Variables|Default|SetLastMoveNormal (Math|Vector|Normalize (Transformation|GetVelocity))))

(event EventTakeDamage
  (params (Damage :type Float%20%28single-precision%29) (IncomingVector :type Vector :default "0, 0, 0") (Attacker :type GLOOM%20Controller%20Object%20Reference) (DamageType :type DamageType%20Enum :default "NewEnumerator4"))
  (|CallParentFunction Damage IncomingVector Attacker DamageType)
  (if (Variables|Default|GetStickingToWall)
    (CallFunction|SetStickingtoWall false "0, 0, 0")))

(event Input|ActionEvents|InputActionJump
  (params (Key :type Key%20Structure))
  (bind _dead (Variables|Default|GetDead))
  (bind _returnvalue (not _dead))
  (:Pressed
    (if _returnvalue
      (Variables|Default|SetHoldingJump true)
      (if (and (not (AI|Components|NavMovement|IsFalling (Variables|Character|GetCharacterMovement))) (not (Variables|Default|GetCrouching)))
        (CallFunction|SetJumpingState true))
      (else
        (CallFunction|ShowClassMenu))))
  (:Released
    (if _returnvalue
      (Variables|Default|SetHoldingJump false)
      (CallFunction|SetJumpingState false)
      (if (Variables|Default|GetStickingToWall)
        (CallFunction|SetStickingtoWall false "0, 0, 0")))))

(event Input|ActionEvents|InputActionPrimeAttack
  (params (Key :type Key%20Structure))
  (:Pressed
    (if (not (Variables|Default|GetDead))
      (if (or (not (AI|Components|NavMovement|IsFalling (Variables|Character|GetCharacterMovement))) (Variables|Default|GetStickingToWall))
        (CallFunction|LaunchAttack)
        (if (Variables|Default|GetStickingToWall)
          (CallFunction|SetStickingtoWall false "0, 0, 0")))
      (else
        (CallFunction|ShowClassMenu)))))

(event Input|AxisEvents|InputAxisLookUp
  (params (AxisValue :type Float%20%28single-precision%29))
  (bind _scenehead (Variables|Default|GetSceneHead))
  (bind _relativerotation (Variables|/Script/Engine.SceneComponent|GetRelativeRotation _scenehead))
  (if (not (Variables|Default|GetDead))
    (Transformation|SetRelativeRotation _scenehead (Math|Rotator|MakeRotator (.roll _relativerotation) (Math|Float|Clamp(Float) (+ (.pitch _relativerotation) (* AxisValue (Variables|Default|GetLookSensitivity))) -89.0 89.0) (.yaw _relativerotation)) false false)))

(event Input|AxisEvents|InputAxisLookRight
  (params (AxisValue :type Float%20%28single-precision%29))
  (if (not (Variables|Default|GetDead))
    (Pawn|Input|AddControllerYawInput (* AxisValue (Variables|Default|GetLookSensitivity) 0.5))))

(event Input|AxisEvents|InputAxisMoveForward
  (params (AxisValue :type Float%20%28single-precision%29))
  (if (not (Variables|Default|GetDead))
    (Class|PawnMovementComponent|AddInputVector (Variables|Character|GetCharacterMovement) (* (Transformation|GetActorForwardVector) AxisValue) false)))

(event Input|AxisEvents|InputAxisMoveRight
  (params (AxisValue :type Float%20%28single-precision%29))
  (if (not (Variables|Default|GetDead))
    (Class|PawnMovementComponent|AddInputVector (Variables|Character|GetCharacterMovement) (* (Transformation|GetActorRightVector) AxisValue) false)))

(fn ConstructionScript
  (|CallParentFunction)
  (bind _returnvalue (AddComponent|AddSceneComponent false))
  (bind _output_get (Variables|Default|SetRotationPoint _returnvalue))
  (Transformation|AttachComponentToComponent _output_get (Variables|Default|GetCapsuleComponent) "None" "KeepRelative" "KeepRelative" "KeepRelative" true)
  (Transformation|AttachComponentToComponent (Variables|Default|GetSceneHead) (Variables|Default|GetRotationPoint) "None" "KeepRelative" "KeepRelative" "KeepRelative" true))

(fn LaunchAttack
  (bind _camera (Variables|Default|GetCamera))
  (bind _returnvalue (Math|Vector|GetForwardVector _camera))
  (Variables|/Script/Engine.CharacterMovementComponent|SetGravityScale (Variables|Character|GetCharacterMovement) (Variables|Default|GetNormalGravityScale))
  (Character|LaunchCharacter (* (Math|Vector|Lerp(Vector) _returnvalue "0, 0,1.000000" (Math|Float|Lerp 0.2 0.0 (Math|Float|Absolute(Float) (Math|Vector|DotProduct _returnvalue "0, 0,1.000000")))) 1.7e+03) false false))

(fn SetStickingtoWall
  (params (StickingToWall :type Boolean) (WallNormal :type Vector))
  (bind _charactermovement (Variables|Character|GetCharacterMovement))
  (bind _output_get (Variables|Default|SetStickingToWall StickingToWall))
  (if _output_get
    (Variables|/Script/Engine.CharacterMovementComponent|SetGravityScale _charactermovement 0.0)
    (Variables|/Script/Engine.MovementComponent|SetVelocity _charactermovement "0, 0, 0")
    (Variables|/Script/Engine.CharacterMovementComponent|SetMaxWalkSpeed _charactermovement 0.0)
    (Variables|Default|SetJumping false)
    (else
      (Variables|/Script/Engine.CharacterMovementComponent|SetGravityScale (Variables|Character|GetCharacterMovement) (Variables|Default|GetNormalGravityScale))
      (CallFunction|ChangeStance (.StanceNormal (Utilities|Struct|BreakClassData (Variables|Default|GetClassData)))))))