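; Alien Wraith player character that can fly while at full health and regenerates after taking damage.
; Pressing jump in midair starts flight and holding it adds lift, while crouching or landing ends it; when dead, jump opens the class menu.
; Damage cancels flight and starts a short delay before Tick restores health, resuming flight at full health if jump is still held while falling.
; SetFlying centralizes the health gate, gravity and movement mode switching.
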(event EventTakeDamage
  (params (Damage :type Float%20%28single-precision%29) (IncomingVector :type Vector :default "0, 0, 0") (Attacker :type GLOOM%20Controller%20Object%20Reference) (DamageType :type DamageType%20Enum :default "NewEnumerator4"))
  (|CallParentFunction Damage IncomingVector Attacker DamageType)
  (Utilities|FlowControl|Sequence
    (:then_0
      (if (Variables|Default|GetFlying)
        (CallFunction|SetFlying false)))
    (:then_1
      (Variables|Default|SetAutoHealTime (+ (Utilities|Time|GetGameTimeinSeconds) 1.0))
      (Variables|Default|SetHurt true))))

(event EventOnLanded
  (params (Hit :type Hit%20Result%20Structure%20%28by%20ref%29))
  (|CallParentFunction Hit)
  (CallFunction|SetFlying false))

(event EventTick
  (params (DeltaSeconds :type Float%20%28single-precision%29))
  (bind _classdata (Variables|Default|GetClassData))
  (bind _health (Utilities|Struct|BreakClassData _classdata))
  (|CallParentFunction DeltaSeconds)
  (Utilities|FlowControl|Sequence
    (:then_0
      (if (and (Variables|Default|GetFlying) (Variables|Default|GetJumpHeld))
        (Class|PawnMovementComponent|AddInputVector (Variables|Character|GetCharacterMovement) "0, 0,1.000000" false)))
    (:then_1
      (if (Variables|Default|GetHurt)
        (if (and (>= (Utilities|Time|GetGameTimeinSeconds) (Variables|Default|GetAutoHealTime)) (not (Variables|Default|GetDead)))
          (Variables|Default|SetHealthCurrent (Math|Float|Min(Float) (+ (* (Utilities|Time|GetWorldDeltaSeconds) 2e+01) (Variables|Default|GetHealthCurrent)) _health))
          (if (== (Variables|Default|GetHealthCurrent) _health)
            (Variables|Default|SetHurt false)
            (if (and (AI|Components|NavMovement|IsFalling (Variables|Character|GetCharacterMovement)) (Variables|Default|GetJumpHeld))
              (CallFunction|SetFlying true))))))))

(event Input|ActionEvents|InputActionJump
  (params (Key :type Key%20Structure))
  (bind _dead (Variables|Default|GetDead))
  (bind _returnvalue (not _dead))
  (:Pressed
    (if _returnvalue
      (Variables|Default|SetJumpHeld true)
      (if (not (AI|Components|NavMovement|IsFalling (Variables|Character|GetCharacterMovement)))
        (CallFunction|SetJumpingState true)
        (else
          (CallFunction|SetJumpingState false)
          (CallFunction|SetFlying true)))
      (else
        (bind _asgloom_hud (Utilities|Casting|CastToGLOOM_HUD (HUD|GetHUD (Game|GetPlayerController 0))))
        (Default|ShowClassMenu _asgloom_hud "NewEnumerator0"))))
  (:Released
    (if _returnvalue
      (Variables|Default|SetJumpHeld false)
      (if (not (Variables|Default|GetFlying))
        (CallFunction|SetJumpingState false)))))

(event Input|ActionEvents|InputActionCrouch
  (params (Key :type Key%20Structure))
  (bind _dead (Variables|Default|GetDead))
  (bind _returnvalue (not _dead))
  (:Pressed
    (if _returnvalue
      (Variables|Default|SetCrouching true)
      (if (not (Variables|Default|GetFlying))
        _
        (else
          (CallFunction|SetFlying false)))
      (CallFunction|ChangeCrouchState)))
  (:Released
    (if _returnvalue
      (Variables|Default|SetCrouching false)
      (CallFunction|ChangeCrouchState))))

(fn ConstructionScript
  (|CallParentFunction))

(fn SetFlying
  (params (Flying :type Boolean))
  (bind _output_get (Variables|Default|SetFlying (and Flying (== (Variables|Default|GetHealthCurrent) (.Health (Utilities|Struct|BreakClassData (Variables|Default|GetClassData)))))))
  (if _output_get
    (Variables|Default|SetJumping false)
    (Variables|/Script/Engine.CharacterMovementComponent|SetGravityScale (Variables|Character|GetCharacterMovement) 0.0)
    (Pawn|Components|CharacterMovement|SetMovementMode (Variables|Character|GetCharacterMovement) "MOVE_Flying" 0)
    (else
      (Variables|/Script/Engine.CharacterMovementComponent|SetGravityScale (Variables|Character|GetCharacterMovement) (Variables|Default|GetNormalGravityScale))
      (Pawn|Components|CharacterMovement|SetMovementMode (Variables|Character|GetCharacterMovement) "MOVE_Falling" 0))))