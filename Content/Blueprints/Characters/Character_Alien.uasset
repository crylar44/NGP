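; Alien player character, a child of a shared character class, with its own vision effect, a second attack and stationary healing.
; An AlienVision2 post-process material is applied to the camera, and SecondAttack input drives the second carried weapon while weapon switching is overridden empty.
; Hitting an Alien_Healer starts health and armor restoration each tick until the alien moves.
; ClassData sets the mesh offset and the loadout checked for missing items.
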(event EventSwitchtoWeapon
  (params (SwitchToIndex :type Integer)))

(event EventBeginPlay
  (bind _carriedweapons (Variables|Default|GetCarriedWeapons))
  (bind _output (Utilities|Array|Get(acopy) _carriedweapons 1))
  (|CallParentFunction)
  (Utilities|IsValid _output
    (:Is%20Valid
      (Default|PutUp _output))))

(event Collision|EventHit
  (params (MyComp :type Primitive%20Component%20Object%20Reference) (Other :type Actor%20Object%20Reference) (OtherComp :type Primitive%20Component%20Object%20Reference) (bSelfMoved :type Boolean) (HitLocation :type Vector :default "0, 0, 0") (HitNormal :type Vector :default "0, 0, 0") (NormalImpulse :type Vector :default "0, 0, 0") (Hit :type Hit%20Result%20Structure%20%28by%20ref%29))
  (|CallParentFunction MyComp Other OtherComp bSelfMoved HitLocation HitNormal NormalImpulse Hit)
  (Utilities|Casting|CastToAlien_Healer Other)
  (Variables|Default|SetGettingHealed true))

(event EventTick
  (params (DeltaSeconds :type Float%20%28single-precision%29))
  (bind _returnvalue (Utilities|Time|GetWorldDeltaSeconds))
  (bind _returnvalue_2 (* _returnvalue 1e+03))
  (|CallParentFunction DeltaSeconds)
  (if (!= (Math|Vector|VectorLength (Transformation|GetVelocity)) 0.0)
    (Variables|Default|SetGettingHealed false)
    (elif (Variables|Default|GetGettingHealed)
      (CallFunction|GetHealed _returnvalue_2)
      (CallFunction|GetRepaired _returnvalue_2))))

(event EventSetUpPostProcessMaterial
  (bind _returnvalue (Rendering|Material|CreateDynamicMaterialInstance "/Game/Materials/PostProcessMaterials/AlienVision2.AlienVision2" :!class /Script/Engine.KismetMaterialLibrary))
  (bind _output_get (Variables|Default|SetPostProcessDynamicMaterial _returnvalue))
  (Variables|/Script/Engine.CameraComponent|SetPostProcessSettings (Variables|Default|GetCamera) (Utilities|Struct|MakePostProcessSettings 1.0 1.7e+02 (Utilities|Struct|MakeWeightedBlendables (Utilities|Array|MakeArray (Utilities|Struct|MakeWeightedBlendable 1.0 _output_get))))))

(event Input|ActionEvents|InputActionSecondAttack
  (params (Key :type Key%20Structure))
  (bind _dead (Variables|Default|GetDead))
  (bind _carriedweapons (Variables|Default|GetCarriedWeapons))
  (bind _returnvalue (not _dead))
  (bind _output (Utilities|Array|Get(acopy) _carriedweapons 1))
  (:Pressed
    (if _returnvalue
      (Utilities|IsValid _output
        (:Is%20Valid
          (Default|TriggerPressed _output)))))
  (:Released
    (if _returnvalue
      (Utilities|IsValid _output
        (:Is%20Valid
          (Default|TriggerReleased _output))))))

(fn ConstructionScript
  (|CallParentFunction)
  (Transformation|SetRelativeLocation (Variables|Default|GetStaticMesh) (Math|Vector|MakeVector 0.0 0.0 (* (.Y (Math|Vector2D|BreakVector2D (Utilities|Struct|BreakStanceData (.StanceNormal (Utilities|Struct|BreakClassData (Variables|Default|GetClassData)))))) -1.0)) false false))

(fn CheckMissingItems
  (bind _classdata (Variables|Default|GetClassData))
  (bind _items (Utilities|Struct|BreakClassData _classdata))
  (LocalVariables|SetMissingItems false)
  (bind _keys (Utilities|Map|Keys _items))
  (for _array_element _keys
    (LocalVariables|SetMissingItems (or (LocalVariables|GetMissingItems) (!= (.Value (Utilities|Map|Find (Variables|Default|GetItems) _array_element)) (.Value (Utilities|Map|Find _items _array_element))))))
  (return (LocalVariables|GetMissingItems)))