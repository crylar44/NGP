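; Human player character Blueprint that adds a human-vision post-process, a toggleable flashlight and ammo and item resupply to its parent class.
; Setup applies a dynamic HumanVision material to the camera, while construction offsets the mesh from the class stance capsule size and randomly rolls the spotlight.
; CheckToRefill reports any weapon or item below class or weapon data amounts; TryRefill restores them and stamps a next-refill time.
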(event Custom|TryRefill
  (Variables|Default|SetRefillAgain (+ (Utilities|Time|GetGameTimeinSeconds) 15.0))
  (Utilities|FlowControl|Sequence
    (:then_0
      (Variables|Default|SetItems (.Items (Utilities|Struct|BreakClassData (Variables|Default|GetClassData)))))
    (:then_1
      (for _array_element (Variables|Default|GetCarriedWeapons)
        (Variables|/Game/Blueprints/Weapons/Weapon.Weapon_C|SetAmmoCarried _array_element (Math|Conversions|ToFloat(Integer) (.AmmoCarrie (Utilities|Struct|BreakWeaponClass (Variables|/Game/Blueprints/Weapons/Weapon.Weapon_C|GetWeaponData _array_element)))))))))

(event EventSetUpPostProcessMaterial
  (bind _returnvalue (Rendering|Material|CreateDynamicMaterialInstance "/Game/Materials/PostProcessMaterials/HumanVision.HumanVision" :!class /Script/Engine.KismetMaterialLibrary))
  (bind _output_get (Variables|Default|SetPostProcessDynamicMaterial _returnvalue))
  (Variables|/Script/Engine.CameraComponent|SetPostProcessSettings (Variables|Default|GetCamera) (Utilities|Struct|MakePostProcessSettings (Utilities|Struct|MakeWeightedBlendables (Utilities|Array|MakeArray (Utilities|Struct|MakeWeightedBlendable 1.0 _output_get))))))

(event Input|ActionEvents|InputActionFlashLight
  (params (Key :type Key%20Structure))
  (bind _spotlight (Variables|Default|GetSpotLight))
  (:Pressed
    (Rendering|SetVisibility _spotlight (not (Variables|/Script/Engine.SceneComponent|GetbVisible _spotlight)) false)))

(fn ConstructionScript
  (|CallParentFunction)
  (Transformation|SetRelativeLocation (Variables|Default|GetStaticMesh) (Math|Vector|MakeVector 0.0 0.0 (* (.Y (Math|Vector2D|BreakVector2D (Utilities|Struct|BreakStanceData (.StanceNormal (Utilities|Struct|BreakClassData (Variables|Default|GetClassData)))))) -1.0)) false false)
  (Transformation|SetRelativeRotation (Variables|Default|GetSpotLight) (Math|Rotator|MakeRotator (Math|Random|RandomFloatinRange 0.0 3.6e+02) 0.0 0.0) false false))

(fn ChecktoRefill
  (Utilities|FlowControl|Sequence
    (:then_0
      (for _array_element (Variables|Default|GetCarriedWeapons)
        (LocalVariables|SetNotFull (or (< (Variables|/Game/Blueprints/Weapons/Weapon.Weapon_C|GetAmmoCarried _array_element) (Math|Conversions|ToFloat(Integer) (Utilities|Struct|BreakWeaponClass (Variables|/Game/Blueprints/Weapons/Weapon.Weapon_C|GetWeaponData _array_element)))) (LocalVariables|GetNotFull)))))
    (:then_1
      (bind _keys (Utilities|Map|Keys (Variables|Default|GetItems)))
      (for _array_element_2 _keys
        (LocalVariables|SetNotFull (or (< (.Value (Utilities|Map|Find (Variables|Default|GetItems) _array_element_2)) (.Value (Utilities|Map|Find (Utilities|Struct|BreakClassData (Variables|Default|GetClassData)) _array_element_2))) (LocalVariables|GetNotFull)))))
    (:then_2
      (return (LocalVariables|GetNotFull)))))