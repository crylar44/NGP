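; Kamikaze Hatchling character Blueprint that adds a hold-to-detonate explosion on the SecondAttack input.
; Pressing sets a trigger flag and restarts a fuse Timeline, while releasing clears the flag without stopping the Timeline.
; If the flag is still set when the Timeline finishes, it spawns a large, high-damage Explosion at the actor's location, credited to GloomController with a fixed team.
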(event Input|ActionEvents|InputActionSecondAttack
  (params (Key :type Key%20Structure))
  (:Pressed
    (Variables|Default|SetEplotionTrigger true)
    (Timeline|TimeTillExplosionIsTriggered PlayFromStart
      (:Finished
        (if (Variables|Default|GetEplotionTrigger)
          (Game|SpawnActorfromClass "/Game/Blueprints/Events/Explosion.Explosion_C" (Math|Conversions|ToTransform(Vector) (Transformation|GetActorLocation)) "Undefined" 0 1.5e+03 1e+03 (Variables|Default|GetGloomController) true true "NewEnumerator1" 0)))))
  (:Released
    (Variables|Default|SetEplotionTrigger false)))

(fn ConstructionScript
  (|CallParentFunction))