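; BioTech human character for GLOOM, a healer that also regenerates its own health shortly after taking damage.
; Holding SecondAttack heals team-filtered characters inside its sphere, while a quick re-press heals one traced target faster; self-regeneration pauses during either.
; Sphere overlaps maintain the group target list and HUD stat tracking.
; It also provides events for its vision post-process material and for capping active flares, destroying the oldest.
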(event OnComponentBeginOverlap(Sphere)
  (params (OverlappedComponent :type Primitive%20Component%20Object%20Reference) (OtherActor :type Actor%20Object%20Reference) (OtherComp :type Primitive%20Component%20Object%20Reference) (OtherBodyIndex :type Integer) (bFromSweep :type Boolean) (SweepResult :type Hit%20Result%20Structure%20%28by%20ref%29))
  (if (!= OtherActor self)
    (bind _asgloom_character (Utilities|Casting|CastToGLOOM_Character OtherActor))
    (if (and (Utilities|Enum|Equal(Enum) (.Team (Utilities|Struct|BreakClassData (Variables|/Game/Blueprints/Characters/GLOOM_Character.GLOOM_Character_C|GetClassData _asgloom_character))) "NewEnumerator2") (not (Utilities|Array|ContainsItem (Variables|Default|GetGroupHealTargets) _asgloom_character)))
      (Utilities|Array|Add (Variables|Default|GetGroupHealTargets) _asgloom_character)
      (bind _gloomcontroller (Variables|Default|GetGloomController)
        (:then
          (Default|TrackActorStats (Variables|/Game/System/GLOOM_Controller.GLOOM_Controller_C|GetGloomHUD _gloomcontroller) _asgloom_character))
        (:else)))))

(event OnComponentEndOverlap(Sphere)
  (params (OverlappedComponent :type Primitive%20Component%20Object%20Reference) (OtherActor :type Actor%20Object%20Reference) (OtherComp :type Primitive%20Component%20Object%20Reference) (OtherBodyIndex :type Integer))
  (bind _asgloom_character (Utilities|Casting|CastToGLOOM_Character OtherActor))
  (if (Utilities|Array|ContainsItem (Variables|Default|GetGroupHealTargets) _asgloom_character)
    (Utilities|Array|RemoveItem (Variables|Default|GetGroupHealTargets) _asgloom_character)
    (bind _gloomcontroller (Variables|Default|GetGloomController)
      (:then
        (Default|StopTrackingActorStats (Variables|/Game/System/GLOOM_Controller.GLOOM_Controller_C|GetGloomHUD _gloomcontroller) _asgloom_character))
      (:else))))

(event Custom|CheckUpOnFlares
  (params (NewFlare :type Grenade%20Flare%20Object%20Reference%20%28by%20ref%29))
  (bind _flaresout (Variables|Default|GetFlaresOut))
  (Utilities|FlowControl|Sequence
    (:then_0
      (if (== (Utilities|Array|Length (Variables|Default|GetFlaresOut)) 4)
        (Actor|DestroyActor (Utilities|Array|Get(acopy) _flaresout))
        (Utilities|Array|RemoveIndex _flaresout)))
    (:then_1
      (Utilities|Array|Add (Variables|Default|GetFlaresOut) NewFlare))))

(event EventSetUpPostProcessMaterial
  (bind _returnvalue (Rendering|Material|CreateDynamicMaterialInstance "/Game/Materials/PostProcessMaterials/HumanVision_BioTech.HumanVision_BioTech" :!class /Script/Engine.KismetMaterialLibrary))
  (bind _output_get (Variables|Default|SetPostProcessDynamicMaterial _returnvalue))
  (Variables|/Script/Engine.CameraComponent|SetPostProcessSettings (Variables|Default|GetCamera) (Utilities|Struct|MakePostProcessSettings (Utilities|Struct|MakeWeightedBlendables (Utilities|Array|MakeArray (Utilities|Struct|MakeWeightedBlendable 1.0 _output_get))))))

(event EventTick
  (params (DeltaSeconds :type Float%20%28single-precision%29))
  (|CallParentFunction DeltaSeconds)
  (if (or (Variables|Default|GetHealingGroup) (Variables|Default|GetHealingSingle))
    (CallFunction|TickHealOthers)
    (else
      (CallFunction|TickAutoHeal))))

(event EventTakeDamage
  (params (Damage :type Float%20%28single-precision%29) (IncomingVector :type Vector :default "0, 0, 0") (Attacker :type GLOOM%20Controller%20Object%20Reference) (DamageType :type DamageType%20Enum :default "NewEnumerator4"))
  (|CallParentFunction Damage IncomingVector Attacker DamageType)
  (Variables|Default|SetAutoHealTime (+ (Utilities|Time|GetGameTimeinSeconds) 1.0))
  (Variables|Default|SetHurt true))

(event Input|ActionEvents|InputActionSecondAttack
  (params (Key :type Key%20Structure))
  (:Pressed
    (if (>= (Utilities|Time|GetGameTimeinSeconds) (Variables|Default|GetHealStartTime))
      (Variables|Default|SetHealStartTime (+ (Utilities|Time|GetGameTimeinSeconds) 0.2))
      (Variables|Default|SetHealingGroup true)
      (else
        (Variables|Default|SetHealingSingle true))))
  (:Released
    (Variables|Default|SetHealingSingle false)
    (Variables|Default|SetHealingGroup false)))

(fn ConstructionScript
  (|CallParentFunction))

(fn TickAutoHeal
  (bind _classdata (Variables|Default|GetClassData))
  (bind _health (Utilities|Struct|BreakClassData _classdata))
  (if (Variables|Default|GetHurt)
    (if (and (>= (Utilities|Time|GetGameTimeinSeconds) (Variables|Default|GetAutoHealTime)) (not (Variables|Default|GetDead)))
      (Variables|Default|SetHealthCurrent (Math|Float|Min(Float) (+ (* (Utilities|Time|GetWorldDeltaSeconds) 2e+01) (Variables|Default|GetHealthCurrent)) _health))
      (if (== (Variables|Default|GetHealthCurrent) _health)
        (Variables|Default|SetHurt false)))))

(fn TickHealOthers
  (bind _camera (Variables|Default|GetCamera))
  (bind _returnvalue (Transformation|GetWorldLocation _camera))
  (if (Variables|Default|GetHealingGroup)
    (for _array_element (Variables|Default|GetGroupHealTargets)
      (Default|GetHealed _array_element (* (Utilities|Time|GetWorldDeltaSeconds) 1e+01)))
    (elif (Variables|Default|GetHealingSingle)
      (bind (_outhit _returnvalue_2) (Collision|LineTraceForObjects _returnvalue (+ _returnvalue (* (Math|Vector|GetForwardVector _camera) 512.0)) (Utilities|Array|MakeArray "ObjectTypeQuery1" "ObjectTypeQuery3") false 0 "None"))
      (if _returnvalue_2
        (bind _asgloom_character (Utilities|Casting|CastToGLOOM_Character (.HitActor (Collision|BreakHitResult _outhit))))
        (if (Utilities|Enum|Equal(Enum) (.Team (Utilities|Struct|BreakClassData (Variables|/Game/Blueprints/Characters/GLOOM_Character.GLOOM_Character_C|GetClassData _asgloom_character))) "NewEnumerator2")
          (Default|GetHealed _asgloom_character (* (Utilities|Time|GetWorldDeltaSeconds) 2e+01)))))))