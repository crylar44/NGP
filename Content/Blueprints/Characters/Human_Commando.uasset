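; Commando human character, a child of a shared character Blueprint, that adds a primed C4 charge to the inherited item system.
; PrimeC4 sets a flag that makes the next UseItem spawn C4 at the character's location, crediting GloomController as attacker, instead of running parent item logic.
; Previous and Next item cycling is blocked while primed.
; An unconnected chain holds alternative priming logic with an item count check and weapon-use delay.
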(event Custom|PrimeC4
  (Variables|Default|SetC4Primed true))

(event EventUseItem
  (params (ItemDataRowName :type Name :default "None"))
  (if (not (Variables|Default|GetC4Primed))
    (|CallParentFunction ItemDataRowName)
    (else
      (Variables|Default|SetC4Primed false)
      (Game|SpawnActorfromClass "/Game/Blueprints/Actors/C4.C4_C" (Math|Transform|MakeTransform (Transformation|GetActorLocation) "0, 0, 0" "1,1,1") "Undefined" 0 (Variables|Default|GetGloomController) 0))))

(event EventTick
  (params (DeltaSeconds :type Float%20%28single-precision%29))
  (|CallParentFunction DeltaSeconds))

(event Input|ActionEvents|InputActionPrevious
  (params (Key :type Key%20Structure))
  (:Pressed
    (if (not (Variables|Default|GetC4Primed))
      (CallFunction|CycleSelectedItem true))))

(event Input|ActionEvents|InputActionNext
  (params (Key :type Key%20Structure))
  (:Pressed
    (if (not (Variables|Default|GetC4Primed))
      (CallFunction|CycleSelectedItem false))))

(fn ConstructionScript
  (|CallParentFunction))