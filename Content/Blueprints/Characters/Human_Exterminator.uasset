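; Exterminator player character whose first weapon, a Photon Cannon, doubles as the shared energy pool for its jetpack and power shield.
; Holding Jump in the air adds lift after a short delay, while jumping from a crouch starts a fast forward boost, both draining that energy each Tick.
; Toggling the shield empties the energy; while on, it halves damage, drains energy per hit and blocks jetpack lift and new boosts.
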(event Custom|TogglePowerShield
  (bind _energysource (Variables|Default|GetEnergySource))
  (Variables|Default|SetPowerShield (not (Variables|Default|GetPowerShield)))
  (Variables|/Game/Blueprints/Weapons/Weapon.Weapon_C|SetAmmoLoaded _energysource 0.0)
  (Default|DelayRecharging _energysource 1.0)
  (Rendering|Material|SetScalarParameterValue (Variables|Default|GetPostProcessDynamicMaterial) "PowerShield" (Math|Conversions|ToFloat(Boolean) (Variables|Default|GetPowerShield)) :!class /Script/Engine.MaterialInstanceDynamic))

(event EventTick
  (params (DeltaSeconds :type Float%20%28single-precision%29))
  (|CallParentFunction DeltaSeconds)
  (CallFunction|TickJetPack))

(event EventSetUpStartWeapons
  (|CallParentFunction)
  (bind _asshooter_photon_cannon (Utilities|Casting|CastToShooter_PhotonCannon (Utilities|Array|Get(acopy) (Variables|Default|GetCarriedWeapons))))
  (Variables|Default|SetEnergySource _asshooter_photon_cannon))

(event EventTakeDamage
  (params (Damage :type Float%20%28single-precision%29) (IncomingVector :type Vector :default "0, 0, 0") (Attacker :type GLOOM%20Controller%20Object%20Reference) (DamageType :type DamageType%20Enum :default "NewEnumerator4"))
  (bind _returnvalue (* Damage 0.5))
  (bind _energysource (Variables|Default|GetEnergySource))
  (if (Variables|Default|GetPowerShield)
    (|CallParentFunction _returnvalue IncomingVector Attacker "NewEnumerator4")
    (Default|CostEnergy _energysource _returnvalue)
    (Default|DelayRecharging _energysource 0.5)
    (else
      (|CallParentFunction Damage IncomingVector Attacker "NewEnumerator4"))))

(event EventOnWalkingOffLedge
  (params (PreviousFloorImpactNormal :type Vector%20%28by%20ref%29 :default "0, 0, 0") (PreviousFloorContactNormal :type Vector%20%28by%20ref%29 :default "0, 0, 0") (PreviousLocation :type Vector%20%28by%20ref%29 :default "0, 0, 0") (TimeDelta :type Float%20%28single-precision%29))
  (|CallParentFunction PreviousFloorImpactNormal PreviousFloorContactNormal PreviousLocation TimeDelta)
  (if (Variables|Default|GetBoosting)
    (CallFunction|SetBoosting false)))

(event EventBeginPlay
  (|CallParentFunction))

(event EventChangeCrouchState
  (|CallParentFunction)
  (if (not (Variables|Default|GetCrouching))
    (if (Variables|Default|GetBoosting)
      (CallFunction|SetBoosting false))))

(event Input|ActionEvents|InputActionJump
  (params (Key :type Key%20Structure))
  (bind _dead (Variables|Default|GetDead))
  (bind _returnvalue (not _dead))
  (:Pressed
    (if _returnvalue
      (Variables|Default|SetHoldingJump true)
      (if (not (AI|Components|NavMovement|IsFalling (Variables|Character|GetCharacterMovement)))
        (if (not (Variables|Default|GetCrouching))
          (CallFunction|SetJumpingState true)
          (elif (not (Variables|Default|GetPowerShield))
            (CallFunction|SetBoosting true))))
      (else
        (CallFunction|ShowClassMenu))))
  (:Released
    (if _returnvalue
      (Variables|Default|SetHoldingJump false)
      (CallFunction|SetJumpingState false)
      (if (Variables|Default|GetBoosting)
        (CallFunction|SetBoosting false)))))

(event Input|ActionEvents|InputActionSecondAttack
  (params (Key :type Key%20Structure))
  (bind _energysource (Variables|Default|GetEnergySource))
  (:Pressed
    (Default|SecondTriggerPressed _energysource))
  (:Released
    (Default|SecondTriggerReleased _energysource)))

(fn ConstructionScript
  (|CallParentFunction))

(fn TickJetPack
  (bind _returnvalue (Transformation|GetVelocity))
  (bind _returnvalue_2 (Utilities|Time|GetWorldDeltaSeconds))
  (bind _energysource (Variables|Default|GetEnergySource))
  (bind _energysource_2 (Variables|Default|GetEnergySource))
  (bind (_x _y) (Math|Vector|BreakVector _returnvalue))
  (if (not (Variables|Default|GetBoosting))
    (if (AI|Components|NavMovement|IsFalling (Variables|Character|GetCharacterMovement))
      (if (Math|Boolean|ANDBoolean (Variables|Default|GetHoldingJump) (>= (Utilities|Time|GetGameTimeinSeconds) (+ (Variables|Default|GetJumpTime) 0.3)) (and (> (Variables|/Game/Blueprints/Weapons/Weapon.Weapon_C|GetAmmoLoaded (Variables|Default|GetEnergySource)) 0.0) (not (Variables|Default|GetPowerShield))))
        (Variables|/Script/Engine.MovementComponent|SetVelocity (Variables|Character|GetCharacterMovement) (Math|Vector|Lerp(Vector) _returnvalue (Math|Vector|MakeVector _x _y 1.6e+03) (* _returnvalue_2 3.0)))
        (Default|CostEnergy _energysource (* _returnvalue_2 3e+01))
        (Default|DelayRecharging _energysource 0.1)))
    (elif (and (Variables|Default|GetBoosting) (> (Variables|/Game/Blueprints/Weapons/Weapon.Weapon_C|GetAmmoLoaded (Variables|Default|GetEnergySource)) 0.0))
      (Class|PawnMovementComponent|AddInputVector (Variables|Character|GetCharacterMovement) (* (Transformation|GetActorForwardVector) 2.0) false)
      (Default|CostEnergy _energysource_2 (* (Utilities|Time|GetWorldDeltaSeconds) 3e+01))
      (Default|DelayRecharging _energysource_2 0.5))))

(fn SetBoosting
  (params (Boosting :type Boolean))
  (bind _output_get (Variables|Default|SetBoosting Boosting))
  (if _output_get
    (Variables|/Script/Engine.CharacterMovementComponent|SetMaxWalkSpeed (Variables|Character|GetCharacterMovement) 1.8e+03)
    (else
      (CallFunction|ChangeCrouchState))))