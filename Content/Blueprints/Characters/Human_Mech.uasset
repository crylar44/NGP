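; Player-controlled human mech character that extends its parent with dual-weapon controls and a twin-spotlight flashlight.
; All carried weapons are put up at BeginPlay, secondary attack fires the second weapon, and SwitchtoWeapon is left empty.
; Reload starts on the first weapon, and holding it until a timeline finishes also reloads the second.
; The construction script splays the spotlights slightly in yaw and randomizes each one's roll.
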(event EventBeginPlay
  (|CallParentFunction)
  (for _array_element (Variables|Default|GetCarriedWeapons)
    (Default|PutUp _array_element)))

(event EventSwitchtoWeapon
  (params (SwitchToIndex :type Integer)))

(event Input|ActionEvents|InputActionFlashLight
  (params (Key :type Key%20Structure))
  (:Pressed
    (Rendering|SetVisibility (Variables|Default|GetSpotLight1) (not (Variables|/Script/Engine.SceneComponent|GetbVisible (Variables|Default|GetSpotLight))) false)))

(event Input|ActionEvents|InputActionSecondAttack
  (params (Key :type Key%20Structure))
  (bind _dead (Variables|Default|GetDead))
  (bind _carriedweapons (Variables|Default|GetCarriedWeapons))
  (bind _returnvalue (not _dead))
  (bind _output (Utilities|Array|Get(acopy) _carriedweapons 1))
  (:Pressed
    (if _returnvalue
      (Utilities|IsValid _output
        (:Is%20Valid
          (Default|TriggerPressed _output)))))
  (:Released
    (if _returnvalue
      (Utilities|IsValid _output
        (:Is%20Valid
          (Default|TriggerReleased _output))))))

(event Input|ActionEvents|InputActionReload
  (params (Key :type Key%20Structure))
  (bind _carriedweapons (Variables|Default|GetCarriedWeapons))
  (bind _dead (Variables|Default|GetDead))
  (bind _returnvalue (not _dead))
  (bind _output (Utilities|Array|Get(acopy) _carriedweapons))
  (:Pressed
    (if _returnvalue
      (Variables|Default|SetReloadHeld true)
      (Default|ReloadPressed _output)
      (Timeline|Timeline_0_0 PlayFromStart
        (:Finished
          (if (Variables|Default|GetReloadHeld)
            (Default|ReloadPressed (Utilities|Array|Get(acopy) (Variables|Default|GetCarriedWeapons) 1)))))))
  (:Released
    (if _returnvalue
      (Variables|Default|SetReloadHeld false)
      (Default|ReloadReleased _output))))

(fn ConstructionScript
  (|CallParentFunction)
  (Transformation|SetRelativeRotation (Variables|Default|GetSpotLight1) (Math|Rotator|MakeRotator (Math|Random|RandomFloatinRange 0.0 3.6e+02) 0.0 -5.0) false false)
  (Transformation|SetRelativeRotation (Variables|Default|GetSpotLight) (Math|Rotator|MakeRotator (Math|Random|RandomFloatinRange 0.0 3.6e+02) 0.0 5.0) false false))