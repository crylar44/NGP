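; Test structure actor that links into a chained energy network with other instances of itself, built in the construction script.
; A procedural mesh draws its reach as a polygonal band.
; GetConnections treats auto-charged structures as chain roots, then recursively claims higher-link structures within range and clear line of sight, updating donor and target lists.
; DrawConnections rebuilds particle components as beams to each target.
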(event EventBeginPlay)

(event Collision|EventActorBeginOverlap
  (params (OtherActor :type Actor%20Object%20Reference)))

(event EventTick
  (params (DeltaSeconds :type Float%20%28single-precision%29)))

(fn ConstructionScript
  (CallFunction|CreateEnergyReachMesh)
  (CallFunction|GetConnections))

(fn CreateEnergyReachMesh
  (bind _tris (LocalVariables|GetTris))
  (bind _corners (LocalVariables|GetCorners))
  (bind _vertices (LocalVariables|GetVertices))
  (bind _autputreachkuk (Variables|Stats|GetAutputReachKUK))
  (bind _tris_2 (LocalVariables|GetTris))
  (bind _returnvalue (- _corners 1))
  (Utilities|FlowControl|Sequence
    (:then_0
      (for _index (range 0 (- (LocalVariables|GetCorners) 1))
        (Utilities|Array|Add _vertices (Math|Vector|RotateVectorAroundAxis (Math|Vector|MakeVector _autputreachkuk 0.0 4.0) (* (/ (Math|Conversions|ToFloat(Integer) _index) (Math|Conversions|ToFloat(Integer) (LocalVariables|GetCorners))) 3.6e+02) "0, 0,1.000000"))
        (Utilities|Array|Add _vertices (Math|Vector|RotateVectorAroundAxis (Math|Vector|MakeVector _autputreachkuk 0.0 -4.0) (* (/ (Math|Conversions|ToFloat(Integer) _index) (Math|Conversions|ToFloat(Integer) (LocalVariables|GetCorners))) 3.6e+02) "0, 0,1.000000"))))
    (:then_1
      (for _index_2 (range 0 _returnvalue)
        (Utilities|Array|Add _tris_2 (* _index_2 2))
        (Utilities|Array|Add _tris_2 (+ (* _index_2 2) 1))
        (Utilities|Array|Add _tris_2 (select (== _index_2 _returnvalue) (Class|KismetSystemLibrary|MakeLiteralInteger) (+ (* _index_2 2) 2)))
        (Utilities|Array|Add _tris (select (== _index_2 _returnvalue) (Class|KismetSystemLibrary|MakeLiteralInteger) (+ (* _index_2 2) 2)))
        (Utilities|Array|Add _tris (+ (* _index_2 2) 1))
        (Utilities|Array|Add _tris (select (== _index_2 _returnvalue) (Class|KismetSystemLibrary|MakeLiteralInteger 1) (+ (* _index_2 2) 3)))))
    (:then_2
      (bind _returnvalue_2 (AddComponent|AddProceduralMeshComponent false))
      (Class|ProceduralMeshComponent|CreateMeshSectionLinearColor _returnvalue_2 0 (LocalVariables|GetVertices) (LocalVariables|GetTris) 0 0 0 0 false)
      (Rendering|Material|SetMaterial _returnvalue_2 0 "/Game/Materials/Mesh/StructureReach.StructureReach"))))

(fn GetConnections
  (Utilities|FlowControl|Sequence
    (:then_0
      (if (!= (Variables|Stats|GetAutoChargeKUK) 0.0)
        (Variables|System|SetChainLinkKUK 0)))
    (:then_1
      (Utilities|Array|Clear (Variables|Default|GetTargetsKUK)))
    (:then_2
      (bind _outactors (Actor|GetAllActorsOfClass "StructureConnectionTest_C"))
      (for _array_element _outactors
        (if (<= (Math|Vector|VectorLength (- (Transformation|GetActorLocation _array_element) (Transformation|GetActorLocation))) (Variables|Stats|GetAutputReachKUK))
          (if (!= (Variables|StructureConnectionTest_C|GetChainLinkKUK _array_element) 0)
            (if (> (Variables|StructureConnectionTest_C|GetChainLinkKUK _array_element) (Variables|System|GetChainLinkKUK))
              (bind _returnvalue (Collision|LineTraceForObjects (Transformation|GetActorLocation) (Transformation|GetActorLocation _array_element) (Utilities|Array|MakeArray "ObjectTypeQuery1") false 0 "None"))
              (if (not _returnvalue)
                (Utilities|Array|Add (Variables|Default|GetTargetsKUK) _array_element)
                (for _array_element_2 (Variables|StructureConnectionTest_C|GetDonersKUK _array_element)
                  (if (< (Variables|StructureConnectionTest_C|GetChainLinkKUK _array_element_2) (Variables|System|GetChainLinkKUK))
                    (Utilities|Array|RemoveItem (Variables|StructureConnectionTest_C|GetDonersKUK _array_element) _array_element_2)
                    (Utilities|Array|RemoveItem (Variables|StructureConnectionTest_C|GetTargetsKUK _array_element_2) _array_element)
                    (CallFunction|DrawConnections _array_element_2)))
                (Utilities|Array|Add (Variables|StructureConnectionTest_C|GetDonersKUK _array_element) self)
                (Variables|StructureConnectionTest_C|SetChainLinkKUK _array_element (+ (Variables|System|GetChainLinkKUK) 1))
                (CallFunction|GetConnections _array_element)))))))
    (:then_3
      (CallFunction|DrawConnections))))

(fn DrawConnections
  (for _array_element (Actor|GetComponentsByClass "/Script/Engine.ParticleSystemComponent")
    (Components|DestroyComponent _array_element))
  (for _array_element_2 (Variables|Default|GetTargetsKUK)
    (bind _returnvalue (AddComponent|AddParticleSystemComponent false))
    (Effects|Components|ParticleSystem|SetTemplate _returnvalue "/Game/ParticleSystems/Beams/StructionConnection.StructionConnection")
    (Effects|Components|ParticleSystem|SetVectorParameter _returnvalue "Donort" "0, 0, 0")
    (Effects|Components|ParticleSystem|SetVectorParameter _returnvalue "Target" (- (Transformation|GetActorLocation _array_element_2) (Transformation|GetActorLocation)))))