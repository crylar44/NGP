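; Web actor that builds a procedural web mesh stretched between nearby static world geometry.
; The construction script randomly rolls a radial ring of line traces about the forward axis and stores the hit points as actor-relative corners.
; It triangulates them as a closed fan around the first vertex and applies the Web material.
; With too few hits to form a web, the actor destroys itself.
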(event EventBeginPlay)

(fn ConstructionScript
  (CallFunction|CreateWebMesh))

(fn CreateWebMesh
  (bind _returnvalue (Transformation|GetActorLocation))
  (bind _sides (Variables|Default|GetSides))
  (bind _corners (Variables|Default|GetCorners))
  (bind _tris (Variables|Default|GetTris))
  (bind _returnvalue_2 (Utilities|Array|LastIndex _corners))
  (Variables|Default|SetUpVector (Math|Vector|RotateVectorAroundAxis (Variables|Default|GetUpVector) (Math|Random|RandomFloatinRange 0.0 3.6e+02) (Variables|Default|GetForwardVector)))
  (Utilities|FlowControl|Sequence
    (:then_0
      (Utilities|Array|Add :TargetArray (Variables|Default|GetCorners))
      (for _index (range 0 (- _sides 1))
        (bind (_outhit _returnvalue_3) (Collision|LineTraceForObjects _returnvalue (+ _returnvalue (* (Math|Vector|RotateVectorAroundAxis (Variables|Default|GetUpVector) (* (/ (Math|Conversions|ToFloat(Integer) _index) (Math|Conversions|ToFloat(Integer) _sides)) 3.6e+02) (Variables|Default|GetForwardVector)) 5e+02)) (Utilities|Array|MakeArray "ObjectTypeQuery1") false 0 "None"))
        (if _returnvalue_3
          (Utilities|Array|Add (Variables|Default|GetCorners) (- (.ImpactPoint (Collision|BreakHitResult _outhit)) (Transformation|GetActorLocation))))))
    (:then_1
      (if (> (Utilities|Array|LastIndex (Variables|Default|GetCorners)) 4)
        (Utilities|FlowControl|Sequence
          (:then_0
            (for _index_2 (range 1 _returnvalue_2)
              (Utilities|Array|Add _tris 0)
              (Utilities|Array|Add _tris _index_2)
              (Utilities|Array|Add _tris (select (== _index_2 _returnvalue_2) (Class|KismetSystemLibrary|MakeLiteralInteger 1) (+ _index_2 1)))))
          (:then_1
            (bind _returnvalue_4 (AddComponent|AddProceduralMeshComponent false))
            (Class|ProceduralMeshComponent|CreateMeshSectionLinearColor _returnvalue_4 0 (Variables|Default|GetCorners) (Variables|Default|GetTris) 0 0 0 0 false)
            (Rendering|Material|SetMaterial _returnvalue_4 0 "/Game/Materials/Mesh/Web.Web")))
        (else
          (Actor|DestroyActor))))))