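; Flashbang explosion actor that blinds nearby characters as soon as it spawns.
; On BeginPlay it runs the parent logic, then, on the authority only, gathers the GLOOM_Character actors overlapping it.
; It calls FlashBangBlinded on each one, skipping members of one team as read from the character's ClassData.
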(event EventBeginPlay
  (|CallParentFunction)
  (Networking|SwitchHasAuthority
    (:Authority
      (for _array_element (Collision|GetOverlappingActors "/Game/Blueprints/Characters/GLOOM_Character.GLOOM_Character_C" :!class /Script/Engine.Actor)
        (bind _asgloom_character (Utilities|Casting|CastToGLOOM_Character _array_element))
        (if (Utilities|Enum|NotEqual(Enum) (Utilities|Struct|BreakClassData (Variables|/Game/Blueprints/Characters/GLOOM_Character.GLOOM_Character_C|GetClassData _asgloom_character)) "NewEnumerator2")
          (Default|FlashBangBlinded _asgloom_character 1.0))))))

(fn ConstructionScript
  (|CallParentFunction))