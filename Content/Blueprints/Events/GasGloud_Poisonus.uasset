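; Poisonous gas cloud hazard that deals continuous damage to enemy characters and structures inside its trigger volume.
; Overlap events maintain separate lists of characters and structures, skipping one fixed team and spawner structures.
; Each tick applies frame-time-scaled damage credited to the Attacker: characters take the DamageOverTime rate with a direction pointing away from the cloud, while structures take a hardcoded rate.
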(event OnComponentBeginOverlap(Trigger)
  (params (OverlappedComponent :type Primitive%20Component%20Object%20Reference) (OtherActor :type Actor%20Object%20Reference) (OtherComp :type Primitive%20Component%20Object%20Reference) (OtherBodyIndex :type Integer) (bFromSweep :type Boolean) (SweepResult :type Hit%20Result%20Structure%20%28by%20ref%29))
  (bind _asgloom_character (Utilities|Casting|CastToGLOOM_Character OtherActor)
    (:then
      (if (Utilities|Enum|NotEqual(Enum) (Utilities|Struct|BreakClassData (Variables|/Game/Blueprints/Characters/GLOOM_Character.GLOOM_Character_C|GetClassData _asgloom_character)) "NewEnumerator1")
        (Utilities|Array|AddUnique (Variables|Default|GetOverlappingEnemyCharacters) _asgloom_character)))
    (:CastFailed
      (bind _asgloom_structure (Utilities|Casting|CastToGLOOM_Structure OtherActor))
      (if (and (Utilities|Enum|NotEqual(Enum) (.Team (Utilities|Struct|BreakStructureData (Variables|/Game/Blueprints/Structures/GLOOM_Structure.GLOOM_Structure_C|GetStructureData _asgloom_structure))) "NewEnumerator1") (not (.Spawner (Utilities|Struct|BreakStructureData (Variables|/Game/Blueprints/Structures/GLOOM_Structure.GLOOM_Structure_C|GetStructureData _asgloom_structure)))))
        (Utilities|Array|AddUnique (Variables|Default|GetOverlappingEnemyStructures) _asgloom_structure)))))

(event OnComponentEndOverlap(Trigger)
  (params (OverlappedComponent :type Primitive%20Component%20Object%20Reference) (OtherActor :type Actor%20Object%20Reference) (OtherComp :type Primitive%20Component%20Object%20Reference) (OtherBodyIndex :type Integer))
  (bind _overlappingenemycharacters (Variables|Default|GetOverlappingEnemyCharacters))
  (bind _overlappingenemystructures (Variables|Default|GetOverlappingEnemyStructures))
  (bind _asgloom_character (Utilities|Casting|CastToGLOOM_Character OtherActor)
    (:then
      (if (Utilities|Array|ContainsItem _overlappingenemycharacters _asgloom_character)
        (Utilities|Array|RemoveItem _overlappingenemycharacters _asgloom_character)))
    (:CastFailed
      (bind _asgloom_structure (Utilities|Casting|CastToGLOOM_Structure OtherActor))
      (if (Utilities|Array|ContainsItem _overlappingenemystructures _asgloom_structure)
        (Utilities|Array|RemoveItem _overlappingenemystructures _asgloom_structure)))))

(event EventTick
  (params (DeltaSeconds :type Float%20%28single-precision%29))
  (Utilities|FlowControl|Sequence
    (:then_0
      (for _array_element (Variables|Default|GetOverlappingEnemyCharacters)
        (Default|TakeDamage _array_element (* (Utilities|Time|GetWorldDeltaSeconds) (Variables|Default|GetDamageOverTime)) (Math|Vector|Normalize (- (Transformation|GetActorLocation _array_element) (Transformation|GetActorLocation))) (Variables|Default|GetAttacker) "NewEnumerator0")))
    (:then_1
      (for _array_element_2 (Variables|Default|GetOverlappingEnemyStructures)
        (Default|TakeDamage _array_element_2 (* (Utilities|Time|GetWorldDeltaSeconds) 1.5e+02) (Variables|Default|GetAttacker))))))

(fn ConstructionScript
  (|CallParentFunction))