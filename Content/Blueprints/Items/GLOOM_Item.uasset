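; GLOOM_Item is an item Blueprint that manages a caster's carried count of a named item.
; SpendItem decrements that item's entry in the caster's ItemsCarried map, and CasterCarriesItem reports whether the count is above zero.
; SpendItem does not check the count itself.
; The event graph holds only an unconnected fragment that would call UseItem on the caster's selected weapon, then delay.
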(fn ConstructionScript)

(fn SpendItem
  (bind _caster (Variables|Default|GetCaster))
  (bind _itemname (Variables|Default|GetItemName))
  (bind _itemscarried (Variables|/Game/Blueprints/Characters/GLOOM_Character.GLOOM_Character_C|GetItemsCarried _caster))
  (Utilities|Map|Add _itemscarried _itemname (- (.Value (Utilities|Map|Find _itemscarried _itemname)) 1)))

(fn CasterCarriesItem
  (return (> (.Value (Utilities|Map|Find (Variables|/Game/Blueprints/Characters/GLOOM_Character.GLOOM_Character_C|GetItemsCarried (Variables|Default|GetCaster)) (Variables|Default|GetItemName))) 0)))