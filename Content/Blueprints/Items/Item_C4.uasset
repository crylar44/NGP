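; Item_C4 is the C4 item actor that primes an explosive charge for a commando caster.
; On BeginPlay, if the caster carries the item, it plays the selected weapon's use-item action and waits that duration plus the item's use time.
; It then spends the item, calls PrimeC4 on the caster cast to Human_Commando, and destroys itself.
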(event EventBeginPlay
  (bind _caster (Variables|Default|GetCaster))
  (bind _data (Variables|Default|GetData))
  (bind _usetime (Utilities|Struct|BreakItemData _data))
  (if (CallFunction|CasterCarriesItem)
    (bind _delay (Default|UseItem (Utilities|Array|Get(acopy) (Variables|/Game/Blueprints/Characters/GLOOM_Character.GLOOM_Character_C|GetCarriedWeapons _caster) (Variables|/Game/Blueprints/Characters/GLOOM_Character.GLOOM_Character_C|GetSelectedWeapon _caster)) _usetime))
    (Utilities|FlowControl|Delay (+ _delay _usetime))
    (CallFunction|SpendItem)
    (bind _ashuman_commando (Utilities|Casting|CastToHuman_Commando (Variables|Default|GetCaster)))
    (Default|PrimeC4 _ashuman_commando)
    (Actor|DestroyActor)))

(fn ConstructionScript
  (|CallParentFunction))