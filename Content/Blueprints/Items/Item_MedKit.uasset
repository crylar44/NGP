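; Med kit item actor that heals the character who uses it and then destroys itself.
; On BeginPlay it checks that the caster carries the item and is not at class maximum health, otherwise it is destroyed immediately.
; The selected weapon runs UseItem, and its returned time plus the item's use time delays spending the item and applying a fixed heal.
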(event EventBeginPlay
  (bind _caster (Variables|Default|GetCaster))
  (bind _data (Variables|Default|GetData))
  (bind _caster_2 (Variables|Default|GetCaster))
  (bind _usetime (Utilities|Struct|BreakItemData _data))
  (if (and (CallFunction|CasterCarriesItem) (!= (Variables|/Game/Blueprints/Characters/GLOOM_Character.GLOOM_Character_C|GetHealthCurrent _caster) (Utilities|Struct|BreakClassData (Variables|/Game/Blueprints/Characters/GLOOM_Character.GLOOM_Character_C|GetClassData _caster))))
    (bind _delay (Default|UseItem (Utilities|Array|Get(acopy) (Variables|/Game/Blueprints/Characters/GLOOM_Character.GLOOM_Character_C|GetCarriedWeapons _caster_2) (Variables|/Game/Blueprints/Characters/GLOOM_Character.GLOOM_Character_C|GetSelectedWeapon _caster_2)) _usetime))
    (Utilities|FlowControl|Delay (+ _delay _usetime))
    (CallFunction|SpendItem)
    (Default|GetHealed (Variables|Default|GetCaster) 6e+01)
    (Actor|DestroyActor)
    (else
      (Actor|DestroyActor))))

(fn ConstructionScript
  (|CallParentFunction))