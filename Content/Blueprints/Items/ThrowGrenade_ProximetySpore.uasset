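; Item action Blueprint that throws a proximity spore grenade from the caster's carried weapon.
; On BeginPlay it triggers the selected weapon's UseItem, waits, spends the item, then spawns Grenade_ProximetySpore at the caster's camera with the caster's GloomController as attacker.
; For an Alien_Guardian caster, it passes the new grenade to CheckUpOnSpores, then destroys itself; other casters skip both steps.
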(event EventBeginPlay
  (bind _caster (Variables|Default|GetCaster))
  (bind _data (Variables|Default|GetData))
  (bind _caster_2 (Variables|Default|GetCaster))
  (bind _usetime (Utilities|Struct|BreakItemData _data))
  (bind _delay (Default|UseItem (Utilities|Array|Get(acopy) (Variables|/Game/Blueprints/Characters/GLOOM_Character.GLOOM_Character_C|GetCarriedWeapons _caster_2) (Variables|/Game/Blueprints/Characters/GLOOM_Character.GLOOM_Character_C|GetSelectedWeapon _caster_2)) _usetime))
  (Utilities|FlowControl|Delay (+ _delay _usetime))
  (CallFunction|SpendItem)
  (bind _returnvalue (Game|SpawnActorfromClass "/Game/Blueprints/Projectiles/Grenade_ProximetySpore.Grenade_ProximetySpore_C" (Transformation|GetWorldTransform (Variables|/Game/Blueprints/Characters/GLOOM_Character.GLOOM_Character_C|GetCamera _caster)) "Undefined" 0 (Variables|/Game/Blueprints/Characters/GLOOM_Character.GLOOM_Character_C|GetGloomController _caster) 0))
  (bind _asalien_guardian (Utilities|Casting|CastToAlien_Guardian (Variables|Default|GetCaster)))
  (Default|CheckUponSpores _asalien_guardian _returnvalue)
  (Actor|DestroyActor))

(fn ConstructionScript
  (|CallParentFunction))