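; Energy network manager actor that procedurally builds a random node graph from its Construction Script; gameplay events are empty.
; SpawnSystem scatters points in a sphere as instanced meshes, with the first as a larger source.
; A step-numbered, breadth-first flood links unvisited neighbors within a fixed radius using targeted particle connections, until growth stops or hits the step cap.
; Disconnected leftovers hold earlier linking, debug-drawing and step-map experiments.
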(event EventBeginPlay)

(event Collision|EventActorBeginOverlap
  (params (OtherActor :type Actor%20Object%20Reference)))

(event EventTick
  (params (DeltaSeconds :type Float%20%28single-precision%29)))

(fn ConstructionScript
  (CallFunction|SpawnSystem))

(fn SpawnSystem
  (bind _sources (Variables|Default|GetSources))
  (LocalVariables|SetDEBUGCOLOR (Math|Conversions|ToLinearColor(Vector) (Math|Random|RandomUnitVector)))
  (Utilities|FlowControl|Sequence
    (:then_0
      (for _index (range 0 (- (Class|KismetSystemLibrary|MakeLiteralInteger 512) 1))
        (Utilities|Array|Add (Variables|Default|GetPoints) (* (Math|Random|RandomUnitVector) (* (- 1.0 (Math|Float|Power (Math|Random|RandomFloat) (Math|Trig|GetPI))) 1.5e+03)))))
    (:then_1
      (bind _returnvalue (AddComponent|AddInstancedStaticMeshComponent false))
      (Components|StaticMesh|SetStaticMesh _returnvalue "/Engine/BasicShapes/Sphere.Sphere")
      (for (_array_element _array_index) (Variables|Default|GetPoints)
        (bind _returnvalue_2 (Utilities|Array|Add _sources (== _array_index 0)))
        (Components|InstancedStaticMesh|AddInstance _returnvalue (Math|Transform|MakeTransform _array_element "0, 0, 0" (Math|Conversions|ToVector(Float) (select (Utilities|Array|Get(acopy) _sources _returnvalue_2) 1.2 0.4))))
        (Utilities|Array|Add (Variables|Default|GetSteps) (Math|Conversions|ToInteger(Boolean) (Utilities|Array|Get(acopy) _sources _returnvalue_2)))))
    (:then_2
      (Variables|Default|SetChangeHasBeenMade false :!label _label)
      (for (_array_element_2 _array_index_2) (Variables|Default|GetSteps)
        (if (== _array_element_2 (Variables|Default|GetCurrentStep))
          (for (_array_element_3 _array_index_3) (Variables|Default|GetPoints)
            (if (and (!= _array_index_3 _array_index_2) (== (Utilities|Array|Get(acopy) (Variables|Default|GetSteps) _array_index_3) 0))
              (if (<= (Math|Vector|VectorLength (- _array_element_3 (Utilities|Array|Get(acopy) (Variables|Default|GetPoints) _array_index_2))) 3e+02)
                (Variables|Default|SetChangeHasBeenMade true)
                (Utilities|Array|SetArrayElem (Variables|Default|GetSteps) _array_index_3 (+ (Variables|Default|GetCurrentStep) 1))
                (bind _returnvalue_3 (AddComponent|AddParticleSystemComponent false (Math|Transform|MakeTransform (Utilities|Array|Get(acopy) (Variables|Default|GetPoints) _array_index_2) "0, 0, 0" "1,1,1")))
                (Effects|Components|ParticleSystem|SetTemplate _returnvalue_3 "/Game/ParticleSystems/Beams/StructionConnection.StructionConnection")
                (Effects|Components|ParticleSystem|SetVectorParameter _returnvalue_3 "Target" (- _array_element_3 (Utilities|Array|Get(acopy) (Variables|Default|GetPoints) _array_index_2))))))))
      (if (Variables|Default|GetChangeHasBeenMade)
        (bind _output_get (Variables|Default|SetCurrentStep (+ (Variables|Default|GetCurrentStep) 1)))
        (if (<= _output_get 33)
          (goto _label)
          (else
            (Development|PrintText "Hello")))
        (else
          (Development|PrintText (Utilities|Text|ToText(Integer) (Variables|Default|GetCurrentStep))))))))