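; Ballistic missile projectile that flies along its local up axis at constant speed and explodes on its first hit.
; Each tick it moves with sweep, then re-orients from its last movement delta so the up axis follows travel.
; A separately spawned trail actor follows it until impact, when the missile spawns an explosion actor, ends the trail and destroys itself.
; Pitch-over rotation and emitter-based explosion nodes are left unconnected.
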(event Custom|Explode
  (Variables|Default|SetExploded true)
  (Game|SpawnActorfromClass "/Game/Blueprints/Events/Explosion.Explosion_C" (Math|Transform|MakeTransform (Transformation|GetActorLocation) "0, 0, 0" "1,1,1") "Undefined" 0 2e+02 2e+02 0 true 0)
  (Default|End (Variables|Default|GetTrail))
  (Actor|DestroyActor))

(event EventTick
  (params (DeltaSeconds :type Float%20%28single-precision%29))
  (bind _returnvalue (Transformation|GetActorLocation))
  (Transformation|AddActorLocalOffset (Math|Vector|MakeVector 0.0 0.0 (* (Utilities|Time|GetWorldDeltaSeconds) 3.7e+03)) true false)
  (Transformation|SetActorRotation (Math|Rotator|MakeRotfromXY (Math|Vector|NegateVector (Math|Vector|GetUpVector (Math|Rotator|MakeRotfromXY (- (Transformation|GetActorLocation) (Variables|Default|GetLastPosition)) (Transformation|GetActorRightVector)))) (Transformation|GetActorRightVector)))
  (Variables|Default|SetLastPosition _returnvalue)
  (bind _trail (Variables|Default|GetTrail)
    (:then
      (Transformation|SetActorLocation _trail _returnvalue true false))
    (:else)))

(event EventBeginPlay
  (Variables|Default|SetLastPosition (+ (Math|Vector|NegateVector (Transformation|GetActorForwardVector)) (Transformation|GetActorLocation)))
  (Transformation|SetActorRotation (Math|Rotator|MakeRotfromXY (Math|Vector|NegateVector (Transformation|GetActorUpVector)) (Transformation|GetActorRightVector)))
  (bind _returnvalue (Game|SpawnActorfromClass "/Game/Blueprints/Effects/BigTrailEffect.BigTrailEffect_C" (Math|Transform|MakeTransform (Transformation|GetActorLocation) "0, 0, 0" "1,1,1") "Undefined" 0 0))
  (Variables|Default|SetTrail _returnvalue))

(event Collision|EventHit
  (params (MyComp :type Primitive%20Component%20Object%20Reference) (Other :type Actor%20Object%20Reference) (OtherComp :type Primitive%20Component%20Object%20Reference) (bSelfMoved :type Boolean) (HitLocation :type Vector :default "0, 0, 0") (HitNormal :type Vector :default "0, 0, 0") (NormalImpulse :type Vector :default "0, 0, 0") (Hit :type Hit%20Result%20Structure%20%28by%20ref%29))
  (if (not (Variables|Default|GetExploded))
    (CallFunction|Explode)))

(fn ConstructionScript)