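; Short-lived fire breath projectile that damages GLOOM characters and structures it overlaps.
; A timeline grows the sphere and drives point light intensity, then destroys the actor, while Tick steadily damps the projectile's velocity.
; Overlaps damage enemy characters, and allies conditionally, judged against a hardcoded team.
; Structures take damage only if they are not on that team and are not spawners.
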(event EventBeginPlay
  (bind _size (Timeline|GrowOverTime Play)
    (:Update
      (Transformation|SetRelativeScale3D (Variables|Default|GetSphere) (Math|Conversions|ToVector(Float) (* _size 2.56)))
      (Rendering|Components|Light|SetIntensity (Variables|Default|GetPointLight) (* _size 5e+03)))
    (:Finished
      (Actor|DestroyActor))))

(event EventTick
  (params (DeltaSeconds :type Float%20%28single-precision%29))
  (bind _projectilemovement (Variables|Default|GetProjectileMovement))
  (Variables|/Script/Engine.MovementComponent|SetVelocity _projectilemovement (* (Variables|/Script/Engine.MovementComponent|GetVelocity _projectilemovement) (- 1.0 (* (Utilities|Time|GetWorldDeltaSeconds) 2.0)))))

(event Collision|EventActorBeginOverlap
  (params (OtherActor :type Actor%20Object%20Reference))
  (Utilities|FlowControl|Sequence
    (:then_0
      (bind _asgloom_character (Utilities|Casting|CastToGLOOM_Character OtherActor))
      (bind _dead (Utilities|GetAllegiance _asgloom_character "NewEnumerator1")
        (:Enemy
          (Default|TakeDamage _asgloom_character (Variables|Default|GetDamage) (Transformation|GetActorForwardVector) (Variables|Default|GetAttacker) "NewEnumerator4" :!label _label))
        (:Allie
          (if _dead
            (goto _label)))))
    (:then_1
      (bind _asgloom_structure (Utilities|Casting|CastToGLOOM_Structure OtherActor))
      (if (and (Utilities|Enum|NotEqual(Enum) (.Team (Utilities|Struct|BreakStructureData (Variables|/Game/Blueprints/Structures/GLOOM_Structure.GLOOM_Structure_C|GetStructureData _asgloom_structure))) "NewEnumerator1") (not (.Spawner (Utilities|Struct|BreakStructureData (Variables|/Game/Blueprints/Structures/GLOOM_Structure.GLOOM_Structure_C|GetStructureData _asgloom_structure)))))
        (Default|TakeDamage _asgloom_structure (Variables|Default|GetDamage) (Variables|Default|GetAttacker))))))

(fn ConstructionScript)