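; Spike spore grenade projectile that bursts two seconds after spawning into a ring of damaging Spike actors, then destroys itself.
; Explode spreads spikes around the vertical axis, with a squared random Z giving slight upward tilt weighted toward horizontal.
; Dividing the angle by count minus one makes the first and last spikes share a heading.
; An Explosion spawn is left disconnected and never runs.
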(event Custom|Explode
  (params (NumberOfSpikes :type Integer))
  (bind _returnvalue (- NumberOfSpikes 1))
  (for _index (range 0 _returnvalue)
    (Game|SpawnActorfromClass "/Game/Blueprints/Projectiles/Spike.Spike_C" (Math|Transform|MakeTransform (Transformation|GetActorLocation) (Math|Conversions|RotationFromXVector (Math|Vector|RotateVectorAroundAxis (Math|Vector|MakeVector 1.0 0.0 (* (Math|Float|Power (Math|Random|RandomFloat) 2.0) 0.2)) (* (/ (Math|Conversions|ToFloat(Integer) _index) (Math|Conversions|ToFloat(Integer) _returnvalue)) 3.6e+02) "0, 0,1.000000")) "1,1,1") "Undefined" 0 1.2e+02 (Variables|Default|GetAttacker) 0 0))
  (Actor|DestroyActor))

(event EventBeginPlay
  (Utilities|FlowControl|Delay 2.0)
  (CallFunction|Explode 16))

(fn ConstructionScript
  (|CallParentFunction))