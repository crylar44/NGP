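; SmallRocket is a rocket projectile that detonates on impact.
; It explodes on any hit, or on overlapping a GLOOM_Character or GLOOM_Structure that is not in its IgnoreObjects list.
; Explode spawns a fixed-radius Explosion at the rocket's location, passing on Damage and Attacker with team damage off and a hardcoded team, then destroys the rocket.
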(event Collision|EventHit
  (params (MyComp :type Primitive%20Component%20Object%20Reference) (Other :type Actor%20Object%20Reference) (OtherComp :type Primitive%20Component%20Object%20Reference) (bSelfMoved :type Boolean) (HitLocation :type Vector :default "0, 0, 0") (HitNormal :type Vector :default "0, 0, 0") (NormalImpulse :type Vector :default "0, 0, 0") (Hit :type Hit%20Result%20Structure%20%28by%20ref%29))
  (CallFunction|Explode))

(event Collision|EventActorBeginOverlap
  (params (OtherActor :type Actor%20Object%20Reference))
  (if (not (Utilities|Array|ContainsItem (Variables|Default|GetIgnoreObjects) OtherActor))
    (Utilities|Casting|CastToGLOOM_Character OtherActor
      (:then
        (CallFunction|Explode))
      (:CastFailed
        (Utilities|Casting|CastToGLOOM_Structure OtherActor)
        (CallFunction|Explode)))))

(fn ConstructionScript)

(fn Explode
  (Game|SpawnActorfromClass "/Game/Blueprints/Events/Explosion.Explosion_C" (Math|Conversions|ToTransform(Vector) (Transformation|GetActorLocation)) "Undefined" 0 1.6e+02 (Variables|Default|GetDamage) (Variables|Default|GetAttacker) true false "NewEnumerator2" 0)
  (Actor|DestroyActor))