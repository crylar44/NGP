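; SpikeSpore_Proximety is a projectile that works as a proximity explosive, sticking where it lands.
; On hitting WorldStatic geometry it zeroes its movement velocity and gravity scale, so it stops in place.
; An overlapping GLOOM_Character triggers Explode unless its ClassData team matches one excluded enum value.
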(event Collision|EventActorBeginOverlap
  (params (OtherActor :type Actor%20Object%20Reference))
  (bind _asgloom_character (Utilities|Casting|CastToGLOOM_Character OtherActor))
  (if (Utilities|Enum|NotEqual(Enum) (Utilities|Struct|BreakClassData (Variables|/Game/Blueprints/Characters/GLOOM_Character.GLOOM_Character_C|GetClassData _asgloom_character)) "NewEnumerator1")
    (CallFunction|Explode 16)))

(event EventBeginPlay)

(event Collision|EventHit
  (params (MyComp :type Primitive%20Component%20Object%20Reference) (Other :type Actor%20Object%20Reference) (OtherComp :type Primitive%20Component%20Object%20Reference) (bSelfMoved :type Boolean) (HitLocation :type Vector :default "0, 0, 0") (HitNormal :type Vector :default "0, 0, 0") (NormalImpulse :type Vector :default "0, 0, 0") (Hit :type Hit%20Result%20Structure%20%28by%20ref%29))
  (bind _projectilemovement (Variables|Default|GetProjectileMovement))
  (if (Utilities|Enum|Equal(Enum) (Collision|GetCollisionObjectType OtherComp) "ECC_WorldStatic")
    (Variables|/Script/Engine.MovementComponent|SetVelocity _projectilemovement "0, 0, 0")
    (Variables|/Script/Engine.ProjectileMovementComponent|SetProjectileGravityScale _projectilemovement 0.0)))

(fn ConstructionScript
  (|CallParentFunction))