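; Poison spit projectile that damages characters and structures not on one specific, hard-coded team.
; Overrides hit events from a parent projectile, crediting each hit to the stored attacker.
; Character hits pass an impact direction away from the projectile and apply a short fixed-length poison, while structure hits deal damage only.
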(event EventHitCharacter
  (params (HitCharacter :type GLOOM%20Character%20Object%20Reference))
  (bind _attacker (Variables|Default|GetAttacker))
  (if (Utilities|Enum|NotEqual(Enum) (.Team (Utilities|Struct|BreakClassData (Variables|/Game/Blueprints/Characters/GLOOM_Character.GLOOM_Character_C|GetClassData HitCharacter))) "NewEnumerator1")
    (Default|TakeDamage HitCharacter (Variables|Default|GetDamage) (Math|Vector|Normalize (- (Transformation|GetActorLocation HitCharacter) (Transformation|GetActorLocation))) _attacker "NewEnumerator4")
    (Default|BecomePoisoned HitCharacter 3.0 _attacker)))

(event EventHitStructure
  (params (HitStructure :type GLOOM%20Structure%20Object%20Reference))
  (if (Utilities|Enum|NotEqual(Enum) (.Team (Utilities|Struct|BreakStructureData (Variables|/Game/Blueprints/Structures/GLOOM_Structure.GLOOM_Structure_C|GetStructureData HitStructure))) "NewEnumerator1")
    (Default|TakeDamage HitStructure (Variables|Default|GetDamage) (Variables|Default|GetAttacker))))

(fn ConstructionScript
  (|CallParentFunction))