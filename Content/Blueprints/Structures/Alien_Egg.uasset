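; Alien Egg structure that acts as a spawn point for one team in the GLOOM game mode.
; On activation it registers with the game mode's team spawns and marks itself ready; being repaid and destroyed while active unregisters it before running the parent logic.
; Each spawn starts a ten-second cooldown, recording the time it will be ready again before re-enabling spawning.
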(event Custom|SpawnClass
  (bind _returnvalue (Math|Float|MakeLiteralFloat 1e+01))
  (Variables|Default|SetReadyToSpawn false)
  (Variables|Default|SetTimeWhenReady (+ (Utilities|Time|GetGameTimeinSeconds) _returnvalue))
  (Utilities|FlowControl|Delay _returnvalue)
  (Variables|Default|SetReadyToSpawn true))

(event EventRepayandDestroy
  (Utilities|FlowControl|Sequence
    (:then_0
      (if (Variables|Default|GetActive)
        (Default|ChangeTeamSpawns (Variables|Default|GetGloomGameMode) "NewEnumerator1" true self)))
    (:then_1
      (|CallParentFunction))))

(event EventActivate
  (|CallParentFunction)
  (Default|ChangeTeamSpawns (Variables|Default|GetGloomGameMode) "NewEnumerator1" false self)
  (Variables|Default|SetReadyToSpawn true))

(event EventBeginPlay
  (|CallParentFunction)
  (bind _asgloom_mode (Utilities|Casting|CastToGLOOM_Mode (Game|GetGameMode)))
  (Variables|Default|SetGloomGameMode _asgloom_mode))

(fn ConstructionScript
  (|CallParentFunction))