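; Alien gaser structure that periodically emits poisonous gas clouds.
; Shortly after BeginPlay it starts ReleaseGas, which spawns a short-lived GasGloud_Poisonus just above the actor, then re-calls itself after a delay to repeat indefinitely.
; Each cloud's projectile movement gets a velocity rotated to a random yaw, so it drifts outward and upward.
; An unconnected loop for spawning several clouds at once never runs.
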(event Custom|ReleaseGas
  (Utilities|FlowControl|Sequence
    (:then_0
      (bind _returnvalue (Game|SpawnActorfromClass "/Game/Blueprints/Events/GasGloud_Poisonus.GasGloud_Poisonus_C" (Math|Conversions|ToTransform(Vector) (+ (Transformation|GetActorLocation) (* (Transformation|GetActorUpVector) 48.0))) "AdjustIfPossibleButAlwaysSpawn" 0 1.5e+02 5.0 2.5e+02 0 0))
      (Variables|/Script/Engine.MovementComponent|SetVelocity (Variables|/Game/Blueprints/Events/GasCloud.GasCloud_C|GetProjectileMovement _returnvalue) (Math|Vector|RotateVectorAroundAxis (Math|Vector|MakeVector 5e+01 0.0 2e+01) (Math|Random|RandomFloatinRange 0.0 3.6e+02) "0, 0,1.000000")))
    (:then_1
      (Utilities|FlowControl|Delay 8.0)
      (CallFunction|ReleaseGas))))

(event EventBeginPlay
  (|CallParentFunction)
  (Utilities|FlowControl|Delay 1.0)
  (CallFunction|ReleaseGas))

(fn ConstructionScript
  (|CallParentFunction))