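; Alien structure that heals, repairs and resupplies alien characters standing within its capsule.
; Capsule overlaps add and remove characters in HealTargets, and Tick restores their health and armor at a fixed per-second rate and refills their items.
; Ticking is enabled on demand, staying on only while targets remain or the structure is damaged.
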(event OnComponentBeginOverlap(Capsule)
  (params (OverlappedComponent :type Primitive%20Component%20Object%20Reference) (OtherActor :type Actor%20Object%20Reference) (OtherComp :type Primitive%20Component%20Object%20Reference) (OtherBodyIndex :type Integer) (bFromSweep :type Boolean) (SweepResult :type Hit%20Result%20Structure%20%28by%20ref%29))
  (bind _ascharacter_alien (Utilities|Casting|CastToCharacter_Alien OtherActor))
  (if (not (Utilities|Array|ContainsItem (Variables|Default|GetHealTargets) _ascharacter_alien))
    (Utilities|Array|Add (Variables|Default|GetHealTargets) _ascharacter_alien)
    (Actor|Tick|SetActorTickEnabled true)))

(event OnComponentEndOverlap(Capsule)
  (params (OverlappedComponent :type Primitive%20Component%20Object%20Reference) (OtherActor :type Actor%20Object%20Reference) (OtherComp :type Primitive%20Component%20Object%20Reference) (OtherBodyIndex :type Integer))
  (bind _ascharacter_alien (Utilities|Casting|CastToCharacter_Alien OtherActor))
  (if (Utilities|Array|ContainsItem (Variables|Default|GetHealTargets) _ascharacter_alien)
    (Utilities|Array|RemoveItem (Variables|Default|GetHealTargets) _ascharacter_alien)
    (CallFunction|KeepTickifDamagedorHasTargets)))

(event EventTick
  (params (DeltaSeconds :type Float%20%28single-precision%29))
  (bind _returnvalue (Utilities|Time|GetWorldDeltaSeconds))
  (bind _returnvalue_2 (* _returnvalue 2e+01))
  (|CallParentFunction DeltaSeconds)
  (CallFunction|KeepTickifDamagedorHasTargets)
  (for _array_element (Variables|Default|GetHealTargets)
    (Default|GetHealed _array_element _returnvalue_2)
    (Default|GetRepaired _array_element _returnvalue_2)
    (Default|TryRefillItems _array_element)))

(fn ConstructionScript
  (|CallParentFunction))

(fn KeepTickifDamagedorHasTargets
  (Actor|Tick|SetActorTickEnabled (or (!= (Utilities|Array|Length (Variables|Default|GetHealTargets)) 0) (Variables|Default|GetDamaged))))