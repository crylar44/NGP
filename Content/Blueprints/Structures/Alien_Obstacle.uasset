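; Alien obstacle structure that hurts and knocks back GLOOM characters of other teams when they collide with it.
; On Hit, a team-checked character takes fixed damage and is launched away from the obstacle's origin.
; A per-character map of game-time stamps enforces a brief cooldown between damage hits.
; Hits that fail the cast, team or cooldown check pass to the parent class's Hit handler.
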(event Collision|EventHit
  (params (MyComp :type Primitive%20Component%20Object%20Reference) (Other :type Actor%20Object%20Reference) (OtherComp :type Primitive%20Component%20Object%20Reference) (bSelfMoved :type Boolean) (HitLocation :type Vector :default "0, 0, 0") (HitNormal :type Vector :default "0, 0, 0") (NormalImpulse :type Vector :default "0, 0, 0") (Hit :type Hit%20Result%20Structure%20%28by%20ref%29))
  (bind _asgloom_character (Utilities|Casting|CastToGLOOM_Character Other)
    (:then
      (if (and (Utilities|Enum|NotEqual(Enum) (.Team (Utilities|Struct|BreakClassData (Variables|/Game/Blueprints/Characters/GLOOM_Character.GLOOM_Character_C|GetClassData _asgloom_character))) "NewEnumerator1") (or (and (<= (.Value (Utilities|Map|Find (Variables|Default|GetTimePassedAllowingToDamage) _asgloom_character)) (Utilities|Time|GetGameTimeinSeconds)) (.ReturnValue (Utilities|Map|Find (Variables|Default|GetTimePassedAllowingToDamage) _asgloom_character))) (not (.ReturnValue (Utilities|Map|Find (Variables|Default|GetTimePassedAllowingToDamage) _asgloom_character)))))
        (Default|TakeDamage _asgloom_character 8e+01 (Math|Vector|Normalize (- (Transformation|GetActorLocation _asgloom_character) (Transformation|GetActorLocation))) 0 "NewEnumerator4")
        (Character|LaunchCharacter _asgloom_character (* (Math|Vector|Normalize (- (Transformation|GetActorLocation _asgloom_character) (Transformation|GetActorLocation))) 5e+01) true true)
        (Utilities|Map|Add (Variables|Default|GetTimePassedAllowingToDamage) _asgloom_character (+ (Utilities|Time|GetGameTimeinSeconds) 0.1))
        (else
          (|CallParentFunction MyComp Other OtherComp bSelfMoved HitLocation HitNormal NormalImpulse Hit :!label _label))))
    (:CastFailed
      (goto _label))))

(fn ConstructionScript
  (|CallParentFunction))