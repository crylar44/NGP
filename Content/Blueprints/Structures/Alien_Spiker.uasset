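; Alien Spiker is an automated turret structure that shoots Spike projectiles at nearby GLOOM characters outside one team.
; A sphere overlap maintains the target list, toggling Tick to save work.
; Tick picks the closest living target not blocked by static geometry and computes direct and velocity-led aim vectors.
; Fire recursively spawns a delayed burst sweeping from near-direct toward led aim as charges deplete, then reloads after a cooldown.
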(event OnComponentBeginOverlap(Sphere)
  (params (OverlappedComponent :type Primitive%20Component%20Object%20Reference) (OtherActor :type Actor%20Object%20Reference) (OtherComp :type Primitive%20Component%20Object%20Reference) (OtherBodyIndex :type Integer) (bFromSweep :type Boolean) (SweepResult :type Hit%20Result%20Structure%20%28by%20ref%29))
  (if (Variables|Default|GetActive)
    (bind _asgloom_character (Utilities|Casting|CastToGLOOM_Character OtherActor))
    (if (and (not (Utilities|Array|ContainsItem (Variables|Default|GetTargetsCloseEnough) _asgloom_character)) (Utilities|Enum|NotEqual(Enum) (.Team (Utilities|Struct|BreakClassData (Variables|/Game/Blueprints/Characters/GLOOM_Character.GLOOM_Character_C|GetClassData _asgloom_character))) "NewEnumerator1"))
      (Utilities|Array|Add (Variables|Default|GetTargetsCloseEnough) _asgloom_character)
      (Actor|Tick|SetActorTickEnabled true))))

(event OnComponentEndOverlap(Sphere)
  (params (OverlappedComponent :type Primitive%20Component%20Object%20Reference) (OtherActor :type Actor%20Object%20Reference) (OtherComp :type Primitive%20Component%20Object%20Reference) (OtherBodyIndex :type Integer))
  (if (Variables|Default|GetActive)
    (bind _asgloom_character (Utilities|Casting|CastToGLOOM_Character OtherActor))
    (if (Utilities|Array|ContainsItem (Variables|Default|GetTargetsCloseEnough) _asgloom_character)
      (Utilities|Array|RemoveItem (Variables|Default|GetTargetsCloseEnough) _asgloom_character)
      (CallFunction|KeepTickifDamagedorHasTargets))))

(event Custom|Fire
  (if (> (Variables|Default|GetCharges) 0)
    (Game|SpawnActorfromClass "/Game/Blueprints/Projectiles/Spike.Spike_C" (Math|Transform|MakeTransform (Transformation|GetWorldLocation (Variables|Default|GetShootPoint)) (Math|Conversions|RotationFromXVector (Math|Vector|Lerp(Vector) (Variables|Default|GetAttackVector) (Variables|Default|GetAttackVectorB) (- 1.0 (/ (Math|Conversions|ToFloat(Integer) (Variables|Default|GetCharges)) 6.0))))) "Undefined" 0 6e+01 0 (Utilities|Array|MakeArray self) 0)
    (Math|Integer|DecrementInt (Variables|Default|GetCharges)
      (:%20%20
        (Utilities|FlowControl|Delay 0.1)
        (CallFunction|Fire)))
    (else
      (Utilities|FlowControl|Delay 3.0)
      (Variables|Default|SetReadyToFire true)
      (Variables|Default|SetCharges 5)
      (CallFunction|KeepTickifDamagedorHasTargets))))

(event EventActivate
  (|CallParentFunction)
  (Variables|Default|SetReadyToFire true)
  (for _array_element (Collision|GetOverlappingActors (Variables|Default|GetSphere) "/Game/Blueprints/Characters/GLOOM_Character.GLOOM_Character_C" :!class /Script/Engine.PrimitiveComponent)
    (bind _asgloom_character (Utilities|Casting|CastToGLOOM_Character _array_element))
    (if (and (not (Utilities|Array|ContainsItem (Variables|Default|GetTargetsCloseEnough) _asgloom_character)) (Utilities|Enum|NotEqual(Enum) (.Team (Utilities|Struct|BreakClassData (Variables|/Game/Blueprints/Characters/GLOOM_Character.GLOOM_Character_C|GetClassData _asgloom_character))) "NewEnumerator1"))
      (Utilities|Array|Add (Variables|Default|GetTargetsCloseEnough) _asgloom_character)
      (Actor|Tick|SetActorTickEnabled true))))

(event EventTick
  (params (DeltaSeconds :type Float%20%28single-precision%29))
  (bind _targetscloseenough (Variables|Default|GetTargetsCloseEnough))
  (bind _returnvalue (Utilities|Array|Length _targetscloseenough))
  (bind _returnvalue_2 (!= _returnvalue 0))
  (|CallParentFunction 0.0)
  (Actor|Tick|SetActorTickEnabled _returnvalue_2)
  (if (and _returnvalue_2 (Variables|Default|GetReadyToFire))
    (Variables|Default|SetTargetFound false)
    (Variables|Default|SetClosestTargetDistance 4096.0)
    (for _array_element (Variables|Default|GetTargetsCloseEnough)
      (if (Variables|/Game/Blueprints/Characters/GLOOM_Character.GLOOM_Character_C|GetDead _array_element)
        (Utilities|Array|RemoveItem (Variables|Default|GetTargetsCloseEnough) _array_element)
        (CallFunction|KeepTickifDamagedorHasTargets)
        (else
          (bind _returnvalue_3 (Collision|LineTraceForObjects (Transformation|GetWorldLocation (Variables|Default|GetShootPoint)) (Transformation|GetActorLocation _array_element) (Utilities|Array|MakeArray "ObjectTypeQuery1") false 0 "None"))
          (if (not _returnvalue_3)
            (Variables|Default|SetTargetFound true)
            (if (> (Variables|Default|GetClosestTargetDistance) (Math|Vector|VectorLength (- (Transformation|GetActorLocation _array_element) (Transformation|GetWorldLocation (Variables|Default|GetShootPoint)))))
              (Variables|Default|SetClosestTargetDistance (Math|Vector|VectorLength (- (Transformation|GetActorLocation _array_element) (Transformation|GetWorldLocation (Variables|Default|GetShootPoint)))))
              (Variables|Default|SetAttackVector (Math|Vector|Normalize (- (Transformation|GetActorLocation _array_element) (Transformation|GetWorldLocation (Variables|Default|GetShootPoint)))))
              (Variables|Default|SetAttackVectorB (Math|Vector|Normalize (- (+ (Transformation|GetActorLocation _array_element) (* (Transformation|GetVelocity _array_element) (* (Utilities|Time|GetWorldDeltaSeconds) 0.01 (Math|Vector|VectorLength (- (Transformation|GetActorLocation _array_element) (Transformation|GetWorldLocation (Variables|Default|GetShootPoint))))))) (Transformation|GetWorldLocation (Variables|Default|GetShootPoint))))))))))
    (if (Variables|Default|GetTargetFound)
      (CallFunction|Fire)
      (Variables|Default|SetReadyToFire false)
      (Actor|Tick|SetActorTickEnabled false)
      (Variables|Default|SetRegenerateTime (+ (Utilities|Time|GetGameTimeinSeconds) 1.0)))))

(fn ConstructionScript
  (|CallParentFunction))

(fn KeepTickifDamagedorHasTargets
  (Actor|Tick|SetActorTickEnabled (or (!= (Utilities|Array|Length (Variables|Default|GetTargetsCloseEnough)) 0) (Variables|Default|GetDamaged))))