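; Base actor for a GLOOM buildable structure that takes damage and refunds team build points when killed or removed.
; Construction loads its data and health from the structure table, then either aligns wall-sticking structures to a nearby surface via sphere trace or sets body physics from the New flag.
; Physics switches off once the body falls asleep.
; Death notifies the attacker, then refunds through GLOOM_Mode and destroys the actor.
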(event OnComponentWake(StructureCoreBody)
  (params (WakingComponent :type Primitive%20Component%20Object%20Reference) (BoneName :type Name :default "None")))

(event OnComponentSleep(StructureCoreBody)
  (params (SleepingComponent :type Primitive%20Component%20Object%20Reference) (BoneName :type Name :default "None"))
  (Physics|SetSimulatePhysics SleepingComponent false))

(event Custom|Die
  (params (Attacker :type GLOOM%20Controller%20Object%20Reference))
  (Default|DestroyedStructure Attacker (Variables|Default|GetDataRowName))
  (CallFunction|RepayandDestroy))

(event Custom|RemoveStructure
  (CallFunction|RepayandDestroy))

(event Custom|TakeDamage
  (params (Damage :type Float%20%28single-precision%29) (Attacker :type GLOOM%20Controller%20Object%20Reference))
  (bind _output_get (Variables|Default|SetHealth (- (Variables|Default|GetHealth) Damage)))
  (if (<= _output_get 0.0)
    (CallFunction|Die Attacker)))

(fn ConstructionScript
  (bind _returnvalue (Transformation|GetActorLocation))
  (bind _structurecorebody (Variables|Default|GetStructureCoreBody))
  (Utilities|FlowControl|Sequence
    (:then_0
      (bind _returnvalue_2 (Utilities|GetDataTableRow "/Game/System/DataTables/StructureTable.StructureTable" (Variables|Default|GetDataRowName))
        (:then
          (bind _output_get (Variables|Default|SetStructureData _returnvalue_2))
          (Variables|Default|SetHealth (Utilities|Struct|BreakStructureData _output_get)))))
    (:then_1
      (if (Utilities|Struct|BreakStructureData (Variables|Default|GetStructureData))
        (Physics|SetSimulatePhysics _structurecorebody false)
        (bind (_outhit _returnvalue_3) (Collision|SphereTraceForObjects _returnvalue _returnvalue 16.0 (Utilities|Array|MakeArray "ObjectTypeQuery1") false 0 "None"))
        (if _returnvalue_3
          (Transformation|SetActorRotation (Math|Rotator|MakeRotfromZ (.ImpactNormal (Collision|BreakHitResult _outhit)))))
        (else
          (Physics|SetSimulatePhysics _structurecorebody (Variables|Default|GetNew)))))))

(fn RegaintheBuildPoints
  (bind _asgloom_mode (Utilities|Casting|CastToGLOOM_Mode (Game|GetGameMode)))
  (Default|ChangeTeamBuildPoints _asgloom_mode (Variables|Default|GetStructureData) true))

(fn RepayandDestroy
  (CallFunction|RegaintheBuildPoints)
  (Actor|DestroyActor))