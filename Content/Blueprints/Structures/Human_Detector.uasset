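; Human structure that detects nearby aliens and signals their presence with a blinking point light.
; Sphere overlap begin and end events add and remove alien characters in a tracked list, then trigger DetectionChange.
; DetectionChange blinks the light through timed delays and calls itself again, looping until the list is empty.
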(event OnComponentBeginOverlap(Sphere)
  (params (OverlappedComponent :type Primitive%20Component%20Object%20Reference) (OtherActor :type Actor%20Object%20Reference) (OtherComp :type Primitive%20Component%20Object%20Reference) (OtherBodyIndex :type Integer) (bFromSweep :type Boolean) (SweepResult :type Hit%20Result%20Structure%20%28by%20ref%29))
  (bind _ascharacter_alien (Utilities|Casting|CastToCharacter_Alien OtherActor))
  (if (not (Utilities|Array|ContainsItem (Variables|Default|GetAliensDetected) _ascharacter_alien))
    (Utilities|Array|Add (Variables|Default|GetAliensDetected) _ascharacter_alien)
    (CallFunction|DetectionChange)))

(event OnComponentEndOverlap(Sphere)
  (params (OverlappedComponent :type Primitive%20Component%20Object%20Reference) (OtherActor :type Actor%20Object%20Reference) (OtherComp :type Primitive%20Component%20Object%20Reference) (OtherBodyIndex :type Integer))
  (bind _ascharacter_alien (Utilities|Casting|CastToCharacter_Alien OtherActor))
  (if (Utilities|Array|ContainsItem (Variables|Default|GetAliensDetected) _ascharacter_alien)
    (Utilities|Array|RemoveItem (Variables|Default|GetAliensDetected) _ascharacter_alien)
    (CallFunction|DetectionChange)))

(event Custom|DetectionChange
  (if (!= (Utilities|Array|Length (Variables|Default|GetAliensDetected)) 0)
    (Rendering|SetVisibility (Variables|Default|GetPointLight) true false)
    (Utilities|FlowControl|Delay 0.5)
    (Rendering|SetVisibility (Variables|Default|GetPointLight) false false)
    (Utilities|FlowControl|Delay 0.2)
    (CallFunction|DetectionChange)))

(fn ConstructionScript
  (|CallParentFunction))