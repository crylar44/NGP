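; Human generator structure that supplies power grid connectivity to other human structures within range.
; A Sphere component defines the range: each Structure_Human entering it receives UpdatePowerGridConnection with this generator as the connection, and each one leaving receives the same call flagged as a disconnect.
; The generator skips itself on begin overlap only, and its construction script just runs the parent's.
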(event OnComponentBeginOverlap(Sphere)
  (params (OverlappedComponent :type Primitive%20Component%20Object%20Reference) (OtherActor :type Actor%20Object%20Reference) (OtherComp :type Primitive%20Component%20Object%20Reference) (OtherBodyIndex :type Integer) (bFromSweep :type Boolean) (SweepResult :type Hit%20Result%20Structure%20%28by%20ref%29))
  (if (!= OtherActor self)
    (bind _asstructure_human (Utilities|Casting|CastToStructure_Human OtherActor))
    (Default|UpdatePowerGridConnection _asstructure_human self false)))

(event OnComponentEndOverlap(Sphere)
  (params (OverlappedComponent :type Primitive%20Component%20Object%20Reference) (OtherActor :type Actor%20Object%20Reference) (OtherComp :type Primitive%20Component%20Object%20Reference) (OtherBodyIndex :type Integer))
  (bind _asstructure_human (Utilities|Casting|CastToStructure_Human OtherActor))
  (Default|UpdatePowerGridConnection _asstructure_human self true))

(fn ConstructionScript
  (|CallParentFunction))