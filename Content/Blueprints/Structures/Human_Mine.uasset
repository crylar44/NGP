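; Human laser tripwire mine structure that arms after its activation delay, showing the beam and enabling its collision.
; Each tick a trace along the up vector resizes the beam capsule and sets the laser material's length up to the first hit.
; A GLOOM character outside the exempt team overlapping the capsule spawns an explosion that spares structures and removes the mine.
; The laser is a procedural one-triangle mesh with a dynamic material, built in construction.
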(event OnComponentBeginOverlap(BeemCollision)
  (params (OverlappedComponent :type Primitive%20Component%20Object%20Reference) (OtherActor :type Actor%20Object%20Reference) (OtherComp :type Primitive%20Component%20Object%20Reference) (OtherBodyIndex :type Integer) (bFromSweep :type Boolean) (SweepResult :type Hit%20Result%20Structure%20%28by%20ref%29))
  (bind _asgloom_character (Utilities|Casting|CastToGLOOM_Character OtherActor))
  (if (Utilities|Enum|NotEqual(Enum) (Utilities|Struct|BreakClassData (Variables|/Game/Blueprints/Characters/GLOOM_Character.GLOOM_Character_C|GetClassData _asgloom_character)) "NewEnumerator2")
    (CallFunction|Explode)))

(event Custom|Explode
  (Game|SpawnActorfromClass "/Game/Blueprints/Events/Explosion.Explosion_C" (Math|Transform|MakeTransform (+ (Transformation|GetActorLocation) (* (Transformation|GetActorForwardVector) 1e+02)) "0, 0, 0" "1,1,1") "Undefined" 0 3e+02 3e+02 0 false true "NewEnumerator0" 0)
  (CallFunction|RemoveStructure))

(event EventBeginPlay
  (|CallParentFunction)
  (Rendering|SetVisibility (Variables|Default|GetLaserMesh) false false)
  (Collision|SetCollisionEnabled (Variables|Default|GetBeemCollision) "NoCollision")
  (Utilities|FlowControl|Delay (.ActivationTime (Utilities|Struct|BreakStructureData (Variables|Default|GetStructureData))))
  (Variables|Default|SetActive true)
  (Collision|SetCollisionEnabled (Variables|Default|GetBeemCollision) "QueryOnly")
  (Actor|Tick|SetActorTickEnabled true)
  (Rendering|SetVisibility (Variables|Default|GetLaserMesh) true false))

(event EventTick
  (params (DeltaSeconds :type Float%20%28single-precision%29))
  (bind _returnvalue (Transformation|GetActorUpVector))
  (bind _returnvalue_2 (Transformation|GetActorLocation))
  (bind _returnvalue_3 (Transformation|GetActorLocation))
  (bind _beemcollision (Variables|Default|GetBeemCollision))
  (bind _returnvalue_4 (* _returnvalue 5e+03))
  (bind _returnvalue_5 (+ _returnvalue_2 _returnvalue_4))
  (bind (_outhit _returnvalue_6) (Collision|LineTraceForObjects (+ _returnvalue_2 (* _returnvalue 15.0)) _returnvalue_5 (Utilities|Array|MakeArray "ObjectTypeQuery1" "ObjectTypeQuery2") false (Utilities|Array|MakeArray self) "None"))
  (Transformation|SetWorldLocation _beemcollision (* (+ _returnvalue_3 (select _returnvalue_6 (.ImpactPoint (Collision|BreakHitResult _outhit)) _returnvalue_5)) 0.5) false false)
  (Components|Capsule|SetCapsuleHalfHeight _beemcollision (* (Math|Vector|VectorLength (- _returnvalue_3 (select _returnvalue_6 (.ImpactPoint (Collision|BreakHitResult _outhit)) _returnvalue_5))) 0.5) true)
  (Rendering|Material|SetScalarParameterValue (Variables|Default|GetLaserMaterial) "Length" (Math|Vector|VectorLength (- _returnvalue_3 (select _returnvalue_6 (.ImpactPoint (Collision|BreakHitResult _outhit)) _returnvalue_5))) :!class /Script/Engine.MaterialInstanceDynamic))

(fn ConstructionScript
  (|CallParentFunction)
  (bind _returnvalue (AddComponent|AddProceduralMeshComponent false))
  (bind _output_get (Variables|Default|SetLaserMesh _returnvalue))
  (Class|ProceduralMeshComponent|CreateMeshSectionLinearColor _output_get 0 (Utilities|Array|MakeArray "0, 0, 0" "0, 0, 0" "0.000000, 0,64.000000" "0.000000,0.000000,4096.000000") (Utilities|Array|MakeArray 0 2 1) 0 (Utilities|Array|MakeArray "(X=0.000000,Y=0.500000)" "(X=1.000000,Y=0.500000)" "" "") 0 0 false)
  (bind _returnvalue_2 (Rendering|Material|CreateDynamicMaterialInstance "/Game/Materials/Mesh/MineLaser.MineLaser" :!class /Script/Engine.KismetMaterialLibrary))
  (bind _output_get_2 (Variables|Default|SetLaserMaterial _returnvalue_2))
  (Rendering|Material|SetMaterial (Variables|Default|GetLaserMesh) 0 _output_get_2)
  (Rendering|Material|SetVectorParameterValue (Variables|Default|GetLaserMaterial) "Forward" (Math|Conversions|ToLinearColor(Vector) (Transformation|GetActorUpVector)) :!class /Script/Engine.MaterialInstanceDynamic))