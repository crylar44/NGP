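; Human power grid node structure that links nearby Structure_Human actors to the grid while it is powered.
; Sphere overlap begin and end events connect or disconnect those structures by passing the node to UpdatePowerGridConnection.
; When the parent UpdatePowerState returns true, the override updates every other overlapping human structure, connecting or disconnecting it to match the node's power state.
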(event OnComponentBeginOverlap(Sphere)
  (params (OverlappedComponent :type Primitive%20Component%20Object%20Reference) (OtherActor :type Actor%20Object%20Reference) (OtherComp :type Primitive%20Component%20Object%20Reference) (OtherBodyIndex :type Integer) (bFromSweep :type Boolean) (SweepResult :type Hit%20Result%20Structure%20%28by%20ref%29))
  (if (Variables|Default|GetPowerd)
    (if (!= OtherActor self)
      (bind _asstructure_human (Utilities|Casting|CastToStructure_Human OtherActor))
      (Default|UpdatePowerGridConnection _asstructure_human self false))))

(event OnComponentEndOverlap(Sphere)
  (params (OverlappedComponent :type Primitive%20Component%20Object%20Reference) (OtherActor :type Actor%20Object%20Reference) (OtherComp :type Primitive%20Component%20Object%20Reference) (OtherBodyIndex :type Integer))
  (if (Variables|Default|GetPowerd)
    (bind _asstructure_human (Utilities|Casting|CastToStructure_Human OtherActor))
    (Default|UpdatePowerGridConnection _asstructure_human self true)))

(fn ConstructionScript
  (|CallParentFunction))

(fn UpdatePowerState
  (bind _newstate (|CallParentFunction))
  (if _newstate
    (for _array_element (Collision|GetOverlappingActors (Variables|Default|GetSphere) "/Game/Blueprints/Structures/Structure_Human.Structure_Human_C" :!class /Script/Engine.PrimitiveComponent)
      (if (!= _array_element self)
        (bind _asstructure_human (Utilities|Casting|CastToStructure_Human _array_element))
        (Default|UpdatePowerGridConnection _asstructure_human self (not (Variables|Default|GetPowerd)))))
    (return true)
    (else
      (return false))))