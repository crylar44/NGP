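; Human teleporter structure that serves as a team spawn point, registered with the GLOOM game mode.
; Pre-placed ones activate on BeginPlay; new ones start inactive until repaired to full health, which also shows the particle effect.
; Repay-and-destroy reports the spawn as lost if active.
; SpawnClass clears ReadyToSpawn as a cooldown, though its Delay uses game time plus ten seconds, so the wait grows over the match.
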(event Custom|SpawnClass
  (bind _returnvalue (Utilities|Time|GetGameTimeinSeconds))
  (bind _returnvalue_2 (Math|Float|MakeLiteralFloat 1e+01))
  (bind _returnvalue_3 (+ _returnvalue _returnvalue_2))
  (Variables|Default|SetReadyToSpawn false)
  (Variables|Default|SetTimeWhenReady _returnvalue_3)
  (Utilities|FlowControl|Delay _returnvalue_3)
  (Variables|Default|SetReadyToSpawn true))

(event EventRepayandDestroy
  (Utilities|FlowControl|Sequence
    (:then_0
      (if (Variables|Default|GetActive)
        (Default|ChangeTeamSpawns (Variables|Default|GetGloomGameMode) "NewEnumerator2" true self)))
    (:then_1
      (|CallParentFunction))))

(event EventRepair
  (|CallParentFunction)
  (if (and (not (Variables|Default|GetActive)) (== (Variables|Default|GetHealth) (Utilities|Struct|BreakStructureData (Variables|Default|GetStructureData))))
    (CallFunction|Activate)
    (CallFunction|ShowParticlesifFullHealth)))

(event EventBeginPlay
  (bind _asgloom_mode (Utilities|Casting|CastToGLOOM_Mode (Game|GetGameMode)))
  (Variables|Default|SetGloomGameMode _asgloom_mode)
  (if (not (Variables|Default|GetNew))
    (CallFunction|Activate)))

(fn ConstructionScript
  (|CallParentFunction)
  (if (Variables|Default|GetNew)
    (Variables|Default|SetHealth 7e+01)
    (Variables|Default|SetActive false)
    (CallFunction|ShowParticlesifFullHealth)))

(fn ShowParticlesifFullHealth
  (Rendering|SetVisibility (Variables|Default|GetParticleSystem) (== (Variables|Default|GetHealth) (Utilities|Struct|BreakStructureData (Variables|Default|GetStructureData))) false))

(fn Activate
  (Variables|Default|SetActive true)
  (Default|ChangeTeamSpawns (Variables|Default|GetGloomGameMode) "NewEnumerator2" false self)
  (Variables|Default|SetReadyToSpawn true))