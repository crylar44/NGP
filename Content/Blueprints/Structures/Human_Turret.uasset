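; Human turret structure that, once repaired to full health, fires rocket bursts at nearby characters outside an excluded team.
; Sphere overlaps maintain the target list and toggle Tick as targets come and go.
; Tick picks the line-of-sight target best aligned with the cannon, using randomized velocity lead, and rotates faster as aim converges.
; When nearly aligned, Fire recursively spawns SmallRocket charges with short delays, then reloads after a cooldown.
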(event OnComponentBeginOverlap(Sphere)
  (params (OverlappedComponent :type Primitive%20Component%20Object%20Reference) (OtherActor :type Actor%20Object%20Reference) (OtherComp :type Primitive%20Component%20Object%20Reference) (OtherBodyIndex :type Integer) (bFromSweep :type Boolean) (SweepResult :type Hit%20Result%20Structure%20%28by%20ref%29))
  (if (Variables|Default|GetActive)
    (bind _asgloom_character (Utilities|Casting|CastToGLOOM_Character OtherActor))
    (if (and (not (Utilities|Array|ContainsItem (Variables|Default|GetTargetsCloseEnough) _asgloom_character)) (Utilities|Enum|NotEqual(Enum) (Utilities|Struct|BreakClassData (Variables|/Game/Blueprints/Characters/GLOOM_Character.GLOOM_Character_C|GetClassData _asgloom_character)) "NewEnumerator2"))
      (Utilities|Array|Add (Variables|Default|GetTargetsCloseEnough) _asgloom_character)
      (Actor|Tick|SetActorTickEnabled true))))

(event OnComponentEndOverlap(Sphere)
  (params (OverlappedComponent :type Primitive%20Component%20Object%20Reference) (OtherActor :type Actor%20Object%20Reference) (OtherComp :type Primitive%20Component%20Object%20Reference) (OtherBodyIndex :type Integer))
  (if (Variables|Default|GetActive)
    (bind _asgloom_character (Utilities|Casting|CastToGLOOM_Character OtherActor))
    (if (and (Utilities|Array|ContainsItem (Variables|Default|GetTargetsCloseEnough) _asgloom_character) (Utilities|Enum|NotEqual(Enum) (Utilities|Struct|BreakClassData (Variables|/Game/Blueprints/Characters/GLOOM_Character.GLOOM_Character_C|GetClassData _asgloom_character)) "NewEnumerator2"))
      (Utilities|Array|RemoveItem (Variables|Default|GetTargetsCloseEnough) _asgloom_character)
      (if (== (Utilities|Array|Length (Variables|Default|GetTargetsCloseEnough)) 0)
        (Actor|Tick|SetActorTickEnabled false)))))

(event Custom|Fire
  (if (> (Variables|Default|GetCharges) 0)
    (Math|Integer|DecrementInt (Variables|Default|GetCharges)
      (:%20%20
        (Game|SpawnActorfromClass "/Game/Blueprints/Projectiles/SmallRocket.SmallRocket_C" (Transformation|GetWorldTransform (Variables|Default|GetCannon)) "Undefined" 0 0 4e+01 (Utilities|Array|MakeArray self) 0)
        (Utilities|FlowControl|Delay 0.2)
        (CallFunction|Fire)))
    (else
      (Utilities|FlowControl|Delay 1.0)
      (Variables|Default|SetReadyToFire true)
      (Variables|Default|SetCharges 3))))

(event EventTick
  (params (DeltaSeconds :type Float%20%28single-precision%29))
  (bind _cannon (Variables|Default|GetCannon))
  (bind _returnvalue (Transformation|GetWorldRotation _cannon))
  (Variables|Default|SetClosestTargetDotProduct 0.0)
  (Variables|Default|SetFoundTarget false)
  (for _array_element (Variables|Default|GetTargetsCloseEnough)
    (if (Variables|/Game/Blueprints/Characters/GLOOM_Character.GLOOM_Character_C|GetDead _array_element)
      (Utilities|Array|RemoveItem (Variables|Default|GetTargetsCloseEnough) _array_element)
      (else
        (bind _returnvalue_2 (Collision|LineTraceForObjects (Transformation|GetWorldLocation (Variables|Default|GetCannon)) (Transformation|GetActorLocation _array_element) (Utilities|Array|MakeArray "ObjectTypeQuery1") false 0 "ForOneFrame"))
        (if (not _returnvalue_2)
          (Variables|Default|SetFoundTarget true)
          (if (< (Variables|Default|GetClosestTargetDotProduct) (* (+ (Math|Vector|DotProduct (Math|Vector|GetForwardVector (Variables|Default|GetCannon)) (Math|Vector|Normalize (- (+ (Transformation|GetActorLocation _array_element) (* (Transformation|GetVelocity _array_element) (* (Utilities|Time|GetWorldDeltaSeconds) (+ (* (Math|Float|Power (Math|Random|RandomFloat) 3.0) 15.0) 1.0)))) (Transformation|GetWorldLocation (Variables|Default|GetCannon))))) 1.0) 0.5))
            (Variables|Default|SetClosestTargetDotProduct (* (+ (Math|Vector|DotProduct (Math|Vector|GetForwardVector (Variables|Default|GetCannon)) (Math|Vector|Normalize (- (+ (Transformation|GetActorLocation _array_element) (* (Transformation|GetVelocity _array_element) (* (Utilities|Time|GetWorldDeltaSeconds) (+ (* (Math|Float|Power (Math|Random|RandomFloat) 3.0) 15.0) 1.0)))) (Transformation|GetWorldLocation (Variables|Default|GetCannon))))) 1.0) 0.5))
            (Variables|Default|SetClosestTargetRotation (Math|Conversions|RotationFromXVector (Math|Vector|Normalize (- (+ (Transformation|GetActorLocation _array_element) (* (Transformation|GetVelocity _array_element) (* (Utilities|Time|GetWorldDeltaSeconds) (+ (* (Math|Float|Power (Math|Random|RandomFloat) 3.0) 15.0) 1.0)))) (Transformation|GetWorldLocation (Variables|Default|GetCannon)))))))))))
  (if (Variables|Default|GetFoundTarget)
    (Transformation|SetWorldRotation (Variables|Default|GetCannon) (Math|Rotator|Lerp(Rotator) _returnvalue (Variables|Default|GetClosestTargetRotation) (Math|Float|Min(Float) (* (/ 1.0 (Math|Vector|VectorLength (- (Math|Vector|GetForwardVector _returnvalue) (Math|Vector|GetForwardVector (Variables|Default|GetClosestTargetRotation))))) (Utilities|Time|GetWorldDeltaSeconds) (Variables|Default|GetTurretRotationSpeed)) 1.0) true) false false)
    (if (and (Variables|Default|GetReadyToFire) (>= (* (/ 1.0 (Math|Vector|VectorLength (- (Math|Vector|GetForwardVector _returnvalue) (Math|Vector|GetForwardVector (Variables|Default|GetClosestTargetRotation))))) (Utilities|Time|GetWorldDeltaSeconds) (Variables|Default|GetTurretRotationSpeed)) 0.9))
      (Variables|Default|SetReadyToFire false)
      (CallFunction|Fire))))

(event EventRepair
  (|CallParentFunction)
  (if (and (not (Variables|Default|GetActive)) (== (Variables|Default|GetHealth) (.Health (Utilities|Struct|BreakStructureData (Variables|Default|GetStructureData)))))
    (bind _output_get (Variables|Default|SetActive true))
    (Rendering|SetVisibility (Variables|Default|GetArrow1) _output_get false)
    (for _array_element (Collision|GetOverlappingActors (Variables|Default|GetSphere) "/Game/Blueprints/Characters/GLOOM_Character.GLOOM_Character_C" :!class /Script/Engine.PrimitiveComponent)
      (bind _asgloom_character (Utilities|Casting|CastToGLOOM_Character _array_element))
      (if (and (not (Utilities|Array|ContainsItem (Variables|Default|GetTargetsCloseEnough) _asgloom_character)) (Utilities|Enum|NotEqual(Enum) (Utilities|Struct|BreakClassData (Variables|/Game/Blueprints/Characters/GLOOM_Character.GLOOM_Character_C|GetClassData _asgloom_character)) "NewEnumerator2"))
        (Utilities|Array|Add (Variables|Default|GetTargetsCloseEnough) _asgloom_character)
        (if (!= (Utilities|Array|Length (Variables|Default|GetTargetsCloseEnough)) 0)
          (Actor|Tick|SetActorTickEnabled true))))))

(fn ConstructionScript
  (|CallParentFunction)
  (if (Variables|Default|GetNew)
    (Variables|Default|SetHealth 3e+02)
    (bind _output_get (Variables|Default|SetActive false))
    (Rendering|SetVisibility (Variables|Default|GetArrow1) _output_get false)))