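; Alien structure Blueprint that activates after spawning and heals itself after taking damage.
; A newly built structure waits for its StructureData activation time before becoming active, while others activate immediately.
; Each hit restarts a one-second regeneration delay and enables Tick, which restores health at a rate derived from StructureData.
; Tick disables itself once health is full, so it runs only while repair is needed.
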(event Custom|Activate
  (Variables|Default|SetActive true))

(event EventTick
  (params (DeltaSeconds :type Float%20%28single-precision%29))
  (bind _structuredata (Variables|Default|GetStructureData))
  (bind (_health _repairrate) (Utilities|Struct|BreakStructureData _structuredata))
  (if (and (Variables|Default|GetDamaged) (>= (Utilities|Time|GetGameTimeinSeconds) (Variables|Default|GetRegenerateTime)))
    (Variables|Default|SetHealth (Math|Float|Min(Float) (+ (Variables|Default|GetHealth) (* (Utilities|Time|GetWorldDeltaSeconds) (/ _health _repairrate))) _health))
    (if (== _health (Variables|Default|GetHealth))
      (Variables|Default|SetDamaged false)
      (Actor|Tick|SetActorTickEnabled false))))

(event EventBeginPlay
  (|CallParentFunction)
  (if (not (Variables|Default|GetNew))
    _
    (else
      (Utilities|FlowControl|Delay (Utilities|Struct|BreakStructureData (Variables|Default|GetStructureData)))))
  (CallFunction|Activate))

(event EventTakeDamage
  (params (Damage :type Float%20%28single-precision%29) (Attacker :type GLOOM%20Controller%20Object%20Reference))
  (|CallParentFunction Damage Attacker)
  (Variables|Default|SetDamaged true)
  (Variables|Default|SetRegenerateTime (+ (Utilities|Time|GetGameTimeinSeconds) 1.0))
  (Actor|Tick|SetActorTickEnabled true))

(fn ConstructionScript
  (|CallParentFunction))