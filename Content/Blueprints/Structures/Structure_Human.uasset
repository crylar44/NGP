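; Human structure Blueprint that handles repair, capped at the structure data's health, and connection to a power grid.
; It tracks sources in range and picks the unobstructed one with the lowest PowerStep, taking one step higher itself when it becomes powered.
; Power state changes swap the core material between emissive and basic.
; While powered, Tick line-traces to the current source and re-evaluates power when the link is blocked.
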(event Custom|Repair
  (bind _structuredata (Variables|Default|GetStructureData))
  (bind (_health _repairrate) (Utilities|Struct|BreakStructureData _structuredata))
  (Variables|Default|SetHealth (Math|Float|Min(Float) _health (+ _repairrate (Variables|Default|GetHealth)))))

(event Custom|UpdatePowerGridConnection
  (params (Connection :type Structure%20Human%20Object%20Reference) (DissConnect :type Boolean))
  (bind _sourcesinrange (Variables|Default|GetSourcesInRange))
  (bind _sourcesinrange_2 (Variables|Default|GetSourcesInRange))
  (bind _returnvalue (Utilities|Array|ContainsItem _sourcesinrange_2 Connection))
  (if (Variables|Default|GetCanBePowerd)
    (Utilities|FlowControl|Sequence
      (:then_0
        (if (not DissConnect)
          (if (not _returnvalue)
            (Utilities|Array|Add _sourcesinrange Connection))
          (elif _returnvalue
            (Utilities|Array|RemoveItem _sourcesinrange Connection))))
      (:then_1
        (CallFunction|UpdatePowerState)))))

(event EventTick
  (params (DeltaSeconds :type Float%20%28single-precision%29))
  (if (Variables|Default|GetPowerd)
    (bind _returnvalue (Collision|LineTraceForObjects (Transformation|GetWorldLocation (Variables|/Game/Blueprints/Structures/GLOOM_Structure.GLOOM_Structure_C|GetStructureCoreBody (Variables|Default|GetCurrentSource))) (Transformation|GetWorldLocation (Variables|Default|GetStructureCoreBody)) (Utilities|Array|MakeArray "ObjectTypeQuery1") false 0 "ForOneFrame"))
    (if _returnvalue
      (CallFunction|UpdatePowerState))))

(fn ConstructionScript
  (|CallParentFunction))

(fn UpdatePowerState
  (bind (_lowestnumberfound _lowestsourcefound _connectionfound) (CallFunction|FindConnectionClosesttoASource))
  (Variables|Default|SetCurrentSource (select _connectionfound _lowestsourcefound 0))
  (if (Math|Boolean|NotEqual(Boolean) _connectionfound (Variables|Default|GetPowerd))
    (bind _output_get (Variables|Default|SetPowerd _connectionfound))
    (Rendering|Material|SetMaterial (Variables|Default|GetStructureCoreBody) 0 (select _output_get "/Game/Materials/EffectMeshMaterials/EmissiveColor.EmissiveColor" "/Engine/BasicShapes/BasicShapeMaterial.BasicShapeMaterial"))
    (Variables|Default|SetPowerStep (select _output_get (+ _lowestnumberfound 1) 100))
    (return true)
    (else
      (return false))))

(fn FindConnectionClosesttoASource
  (if (!= (Utilities|Array|Length (Variables|Default|GetSourcesInRange)) 0)
    (LocalVariables|SetLowestNumber 100)
    (for _array_element (Variables|Default|GetSourcesInRange)
      (bind _returnvalue (Collision|LineTraceForObjects (Transformation|GetWorldLocation (Variables|Default|GetStructureCoreBody)) (Transformation|GetWorldLocation (Variables|/Game/Blueprints/Structures/GLOOM_Structure.GLOOM_Structure_C|GetStructureCoreBody _array_element)) (Utilities|Array|MakeArray "ObjectTypeQuery1") false 0 "ForDuration"))
      (if (and (not _returnvalue) (< (Variables|Structure_Human_C|GetPowerStep _array_element) (LocalVariables|GetLowestNumber)))
        (LocalVariables|SetLowestNumber (Variables|Structure_Human_C|GetPowerStep _array_element))
        (LocalVariables|SetLowestSource _array_element)))
    (return (LocalVariables|GetLowestNumber) (LocalVariables|GetLowestSource) (< (LocalVariables|GetLowestNumber) (Variables|Default|GetPowerStep)))
    (else
      (return 100 0 false))))