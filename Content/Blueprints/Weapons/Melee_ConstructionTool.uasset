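; Melee construction tool weapon that damages enemies and repairs allied characters and human structures.
; On a hit, it casts the object to a character or structure and branches on a team check.
; Enemies and dead allies take damage, while living allies are repaired.
; Enemy structures take damage, spawners only when HurtSpawners is set, and allied Structure_Human actors get repaired.
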(event EventHitObject
  (params (Object :type Object%20Object%20Reference) (Damage :type Float%20%28single-precision%29) (Vector :type Vector :default "0, 0, 0"))
  (bind _asgloom_character (Utilities|Casting|CastToGLOOM_Character Object)
    (:then
      (bind (_dead _holderscontroller) (Utilities|CheckTargetCharacter _asgloom_character)
        (:Enemy
          (Default|TakeDamage _asgloom_character Damage Vector _holderscontroller "NewEnumerator4" :!label _label))
        (:Allie
          (if _dead
            (goto _label)
            (else
              (Default|GetRepaired _asgloom_character 1.0))))))
    (:CastFailed
      (bind _asgloom_structure (Utilities|Casting|CastToGLOOM_Structure Object))
      (bind _holderscontroller_2 (Utilities|CheckTeam (.Team (Utilities|Struct|BreakStructureData (Variables|/Game/Blueprints/Structures/GLOOM_Structure.GLOOM_Structure_C|GetStructureData _asgloom_structure))))
        (:Enemy
          (if (not (.Spawner (Utilities|Struct|BreakStructureData (Variables|/Game/Blueprints/Structures/GLOOM_Structure.GLOOM_Structure_C|GetStructureData _asgloom_structure))))
            (Default|TakeDamage _asgloom_structure Damage _holderscontroller_2)
            (elif (Variables|Default|GetHurtSpawners)
              (Default|TakeDamage _asgloom_structure Damage _holderscontroller_2))))
        (:Allie
          (bind _asstructure_human (Utilities|Casting|CastToStructure_Human _asgloom_structure))
          (Default|Repair _asstructure_human))))))

(fn ConstructionScript
  (|CallParentFunction))