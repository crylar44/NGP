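; Gatling guns weapon Blueprint, a child shooter that fires alternately from a left and a right gun.
; FireAttack runs the parent's attack, then passes the inverted RightGun flag to UpdateMuzzlePoint.
; UpdateMuzzlePoint stores that flag and mirrors the lateral offset of MuzzlePointVector, so the next shot leaves from the opposite side.
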(event EventFireAttack
  (params (Damage :type Float%20%28single-precision%29) (Spread :type Float%20%28single-precision%29))
  (|CallParentFunction Damage Spread)
  (CallFunction|UpdateMuzzlePoint (not (Variables|Default|GetRightGun))))

(fn ConstructionScript
  (|CallParentFunction))

(fn UpdateMuzzlePoint
  (params (RightGun :type Boolean))
  (bind _output_get (Variables|Default|SetRightGun RightGun))
  (Variables|Default|SetMuzzlePointVector (Math|Vector|MakeVector 0.0 (Utilities|Select :Index (Math|Conversions|ToInteger(Boolean) _output_get) :Option%200 -25.0 :Option%201 25.0) -15.0)))