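; Mounted rocket launcher weapon that fires a SmallRocket on each attack, alternating between a right and a left launcher.
; FireAttack spawns the rocket at the muzzle point along the spread-adjusted aim, passing damage and ignoring the holder, then flips sides.
; SetNextLauncher stores the active side and mirrors the muzzle offset laterally; construction starts it on the right.
; An eight-step launcher counter remains as unconnected leftover logic.
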(event EventFireAttack
  (params (Damage :type Float%20%28single-precision%29) (Spread :type Float%20%28single-precision%29))
  (Game|SpawnActorfromClass "/Game/Blueprints/Projectiles/SmallRocket.SmallRocket_C" (Math|Transform|MakeTransform (CallFunction|MuzzlePoint) (Math|Conversions|RotationFromXVector (CallFunction|AimVectorwithSpread Spread))) "Undefined" 0 0 Damage (Utilities|Array|MakeArray (Variables|Default|GetHolder)) 0)
  (CallFunction|SetNextLauncher (not (Variables|Default|GetRightLauncher))))

(fn ConstructionScript
  (|CallParentFunction)
  (CallFunction|SetNextLauncher true))

(fn SetNextLauncher
  (params (RightLauncher :type Boolean))
  (bind _output_get (Variables|Default|SetRightLauncher RightLauncher))
  (Variables|Default|SetMuzzlePointVector (Math|Vector|MakeVector 0.0 (Utilities|Select :Index (Math|Conversions|ToInteger(Boolean) _output_get) :Option%200 -35.0 :Option%201 35.0) 2e+01)))