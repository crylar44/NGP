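; Photon Cannon weapon for GLOOM with a recharging energy pool, normal fire and a secondary-armed discharge shot.
; Holding secondary makes the primary trigger discharge, which hurts the holder, spends energy and lowers maximum charge; otherwise it calls KeepFiring.
; Discharge traces to world geometry, then multi-traces that segment to damage each target once, sparing living allies but not friendly structures.
; HitObject applies team-filtered damage; an older hitscan shot remains unwired.
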(event Custom|Discharge
  (bind _holder (Variables|Default|GetHolder))
  (bind _muzzlepointvector (Variables|Default|GetMuzzlePointVector))
  (bind _holder_2 (Variables|Default|GetHolder))
  (bind _holder_3 (Variables|Default|GetHolder))
  (bind _camera (Variables|/Game/Blueprints/Characters/GLOOM_Character.GLOOM_Character_C|GetCamera _holder))
  (bind _camera_2 (Variables|/Game/Blueprints/Characters/GLOOM_Character.GLOOM_Character_C|GetCamera _holder_2))
  (bind _camera_3 (Variables|/Game/Blueprints/Characters/GLOOM_Character.GLOOM_Character_C|GetCamera _holder_3))
  (bind _returnvalue (Math|Vector|GetForwardVector _camera_2))
  (bind _returnvalue_2 (Transformation|GetWorldLocation _camera_3))
  (bind _returnvalue_3 (* _returnvalue 5e+03))
  (bind _returnvalue_4 (+ _returnvalue_2 _returnvalue_3))
  (Utilities|FlowControl|Sequence
    (:then_0
      (Default|TakeDamage _holder_3 5e+01 "0, 0, 0" (Variables|/Game/Blueprints/Characters/GLOOM_Character.GLOOM_Character_C|GetGloomController _holder_3) "NewEnumerator4")
      (CallFunction|CostEnergy 2e+02)
      (Variables|Default|SetLostMaxEnergy (+ (Variables|Default|GetLostMaxEnergy) 2e+01)))
    (:then_1
      (bind (_outhit _returnvalue_5) (Collision|LineTraceForObjects _returnvalue_2 _returnvalue_4 (Utilities|Array|MakeArray "ObjectTypeQuery1") false 0 "None"))
      (Utilities|FlowControl|Sequence
        (:then_0
          (bind (_outhits _returnvalue_6) (Class|KismetSystemLibrary|LineTraceMultiforObjects _returnvalue_2 (select _returnvalue_5 (.ImpactPoint (Collision|BreakHitResult _outhit)) _returnvalue_4) (Utilities|Array|MakeArray "ObjectTypeQuery3" "ObjectTypeQuery1" "ObjectTypeQuery2" "ObjectTypeQuery4") false (Utilities|Array|MakeArray (Variables|Default|GetHolder)) "None" true))
          (Utilities|Array|Clear (Variables|Default|GetHandledTargets))
          (if _returnvalue_6
            (for _array_element _outhits
              (if (not (Utilities|Array|ContainsItem (Variables|Default|GetHandledTargets) (.HitActor (Collision|BreakHitResult _array_element))))
                (Utilities|Array|Add (Variables|Default|GetHandledTargets) (.HitActor (Collision|BreakHitResult _array_element)))
                (bind _asgloom_structure (Utilities|Casting|CastToGLOOM_Structure (.HitActor (Collision|BreakHitResult _array_element)))
                  (:then
                    (Default|TakeDamage _asgloom_structure (Variables|Default|GetDischargeDamage) (Variables|/Game/Blueprints/Characters/GLOOM_Character.GLOOM_Character_C|GetGloomController (Variables|Default|GetHolder))))
                  (:CastFailed
                    (bind _asgloom_character (Utilities|Casting|CastToGLOOM_Character (.HitActor (Collision|BreakHitResult _array_element))))
                    (bind (_dead _holderscontroller) (Utilities|CheckTargetCharacter _asgloom_character)
                      (:Enemy
                        (Default|TakeDamage _asgloom_character (Variables|Default|GetDischargeDamage) "0, 0, 0" _holderscontroller "NewEnumerator4" :!label _label))
                      (:Allie
                        (if _dead
                          (goto _label))))))))))
        (:then_1
          (Variables|Default|SetFireTime (Utilities|Time|GetGameTimeinSeconds))
          (Game|SpawnActorfromClass "/Game/Blueprints/Effects/TrailEffect.TrailEffect_C" (Math|Transform|MakeTransform (+ (Transformation|GetWorldLocation _camera) (* (Math|Vector|GetForwardVector _camera) (.x _muzzlepointvector)) (* (Math|Vector|GetRightVector _camera) (.y _muzzlepointvector)) (* (Math|Vector|GetUpVector _camera) (.z _muzzlepointvector))) "0, 0, 0" "1,1,1") "Undefined" 0 (select _returnvalue_5 (.ImpactPoint (Collision|BreakHitResult _outhit)) _returnvalue_4) 0))))))

(event Custom|SecondTriggerReleased
  (Variables|Default|SetReadyDischarge false))

(event Custom|SecondTriggerPressed
  (Variables|Default|SetReadyDischarge true))

(event EventHitObject
  (params (Object :type Object%20Object%20Reference) (Damage :type Float%20%28single-precision%29) (Vector :type Vector :default "0, 0, 0") (ImpactPoint :type Vector :default "0, 0, 0") (ImpactNormal :type Vector :default "0, 0, 0"))
  (bind _asgloom_character (Utilities|Casting|CastToGLOOM_Character Object)
    (:then
      (bind (_dead _holderscontroller) (Utilities|CheckTargetCharacter _asgloom_character)
        (:Enemy
          (Default|TakeDamage _asgloom_character Damage (Math|Vector|Normalize Vector) _holderscontroller "NewEnumerator6" :!label _label))
        (:Allie
          (if _dead
            (goto _label)))))
    (:CastFailed
      (bind _asgloom_structure (Utilities|Casting|CastToGLOOM_Structure Object))
      (if (and (Utilities|Enum|NotEqual(Enum) (.Team (Utilities|Struct|BreakStructureData (Variables|/Game/Blueprints/Structures/GLOOM_Structure.GLOOM_Structure_C|GetStructureData _asgloom_structure))) (.Team (Utilities|Struct|BreakClassData (Variables|/Game/Blueprints/Characters/GLOOM_Character.GLOOM_Character_C|GetClassData (Variables|Default|GetHolder))))) (not (.Spawner (Utilities|Struct|BreakStructureData (Variables|/Game/Blueprints/Structures/GLOOM_Structure.GLOOM_Structure_C|GetStructureData _asgloom_structure)))))
        (Default|TakeDamage _asgloom_structure Damage (Variables|/Game/Blueprints/Characters/GLOOM_Character.GLOOM_Character_C|GetGloomController (Variables|Default|GetHolder)))))))

(event EventTickRecharge
  (if (>= (Utilities|Time|GetGameTimeinSeconds) (Variables|Default|GetRechargeStartTime))
    (Variables|Default|SetAmmoLoaded (Math|Float|Min(Float) (- (Math|Conversions|ToFloat(Integer) (.AmmoLoad (Utilities|Struct|BreakWeaponClass (Variables|Default|GetWeaponData)))) (Variables|Default|GetLostMaxEnergy)) (+ (Variables|Default|GetAmmoLoaded) (* (Utilities|Time|GetWorldDeltaSeconds) 1e+01))))))

(event EventTriggerPressed
  (Variables|Default|SetTriggerHeld true)
  (if (Utilities|Enum|Equal(Enum) (Variables|Default|GetWeaponState) "NewEnumerator2")
    (if (not (Variables|Default|GetReadyDischarge))
      (CallFunction|KeepFiring)
      (else
        (CallFunction|Discharge)))))

(event EventTriggerReleased
  (Variables|Default|SetTriggerHeld false))

(fn ConstructionScript
  (|CallParentFunction))

(fn CostEnergy
  (params (Cost :type Float%20%28single-precision%29))
  (bind _output_get (Variables|Default|SetAmmoLoaded (- (Variables|Default|GetAmmoLoaded) Cost)))
  (if (<= _output_get 0.0)
    (CallFunction|DelayRecharging 3.0)
    (Variables|Default|SetAmmoLoaded 0.0)))