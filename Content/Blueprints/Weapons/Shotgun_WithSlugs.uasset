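; Shotgun weapon Blueprint with an alternate explosive slug ammo type, toggled by holding reload.
; A reload press runs the timed reload alongside the CheckReload timeline, which swaps loaded, carried and stashed ammo if reload is still held when it finishes.
; FireAttack defers to the parent for normal shells, while slugs line trace from the camera with random cone spread, spawning an explosion on hit and a trail effect.
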(event Custom|ChangeAmmo
  (Variables|Default|SetSlugsLoaded (not (Variables|Default|GetSlugsLoaded)))
  (Variables|Default|SetAmmoCarried (+ (Variables|Default|GetAmmoLoaded) (Variables|Default|GetAmmoCarried)))
  (Variables|Default|SetAmmoLoaded (Variables|Default|GetAmmoStashed))
  (Variables|Default|SetAmmoStashed (Variables|Default|GetAmmoCarried))
  (Variables|Default|SetAmmoCarried (Variables|Default|GetAmmoLoaded))
  (Variables|Default|SetAmmoLoaded 0.0))

(event EventFireAttack
  (params (Damage :type Float%20%28single-precision%29) (Spread :type Float%20%28single-precision%29))
  (bind _returnvalue (Math|Random|RandomFloatinRange 0.0 3.6e+02))
  (bind _slugs (Variables|Default|GetSlugs))
  (bind _holder (Variables|Default|GetHolder))
  (bind _muzzlepointvector (Variables|Default|GetMuzzlePointVector))
  (bind _holder_2 (Variables|Default|GetHolder))
  (bind _holder_3 (Variables|Default|GetHolder))
  (bind _spread (Utilities|Struct|BreakWeaponClass _slugs))
  (bind _camera (Variables|/Game/Blueprints/Characters/GLOOM_Character.GLOOM_Character_C|GetCamera _holder))
  (bind _camera_2 (Variables|/Game/Blueprints/Characters/GLOOM_Character.GLOOM_Character_C|GetCamera _holder_2))
  (bind _camera_3 (Variables|/Game/Blueprints/Characters/GLOOM_Character.GLOOM_Character_C|GetCamera _holder_3))
  (bind _returnvalue_2 (Math|Vector|GetForwardVector _camera_2))
  (bind _returnvalue_3 (Math|Vector|GetRightVector _camera_2))
  (bind _returnvalue_4 (Math|Random|RandomFloatinRange 0.0 _spread))
  (bind _returnvalue_5 (Transformation|GetWorldLocation _camera_3))
  (bind _returnvalue_6 (Math|Vector|RotateVectorAroundAxis _returnvalue_2 _returnvalue_4 _returnvalue_3))
  (bind _returnvalue_7 (Math|Vector|RotateVectorAroundAxis _returnvalue_6 _returnvalue _returnvalue_2))
  (bind _returnvalue_8 (* _returnvalue_7 5e+03))
  (bind _returnvalue_9 (+ _returnvalue_5 _returnvalue_8))
  (if (not (Variables|Default|GetSlugsLoaded))
    (|CallParentFunction Damage Spread)
    (else
      (bind (_outhit _returnvalue_10) (Collision|LineTraceForObjects _returnvalue_5 _returnvalue_9 (Utilities|Array|MakeArray "ObjectTypeQuery1" "ObjectTypeQuery2" "ObjectTypeQuery3" "ObjectTypeQuery4") false (Utilities|Array|MakeArray (Variables|Default|GetHolder)) "None"))
      (Utilities|FlowControl|Sequence
        (:then_0
          (if _returnvalue_10
            (Game|SpawnActorfromClass "/Game/Blueprints/Events/Explosion.Explosion_C" (Math|Transform|MakeTransform (.ImpactPoint (Collision|BreakHitResult _outhit)) "0, 0, 0" "1,1,1") "Undefined" 0 2e+02 (Utilities|Struct|BreakWeaponClass (Variables|Default|GetSlugs)) (Variables|/Game/Blueprints/Characters/GLOOM_Character.GLOOM_Character_C|GetGloomController (Variables|Default|GetHolder)) true true "NewEnumerator2" 0)))
        (:then_1
          (Variables|Default|SetFireTime (Utilities|Time|GetGameTimeinSeconds))
          (Game|SpawnActorfromClass "/Game/Blueprints/Effects/TrailEffect.TrailEffect_C" (Math|Transform|MakeTransform (+ (Transformation|GetWorldLocation _camera) (* (Math|Vector|GetForwardVector _camera) (.x _muzzlepointvector)) (* (Math|Vector|GetRightVector _camera) (.y _muzzlepointvector)) (* (Math|Vector|GetUpVector _camera) (.z _muzzlepointvector))) "0, 0, 0" "1,1,1") "Undefined" 0 (select _returnvalue_10 (.ImpactPoint (Collision|BreakHitResult _outhit)) _returnvalue_9) 0))))))

(event EventReloadPressed
  (Variables|Default|SetReloadHeld true)
  (if (Utilities|Enum|Equal(Enum) (Variables|Default|GetWeaponState) "NewEnumerator2")
    (Variables|Default|SetWeaponState "NewEnumerator5")
    (Utilities|FlowControl|Sequence
      (:then_0
        (Utilities|FlowControl|Delay (Utilities|Struct|BreakWeaponClass (Variables|Default|GetWeaponData)))
        (CallFunction|LoadAmmo (Variables|Default|GetAmmoLoaded))
        (if (Variables|Default|GetTriggerHeld)
          (CallFunction|KeepFiring)
          (else
            (Variables|Default|SetWeaponState "NewEnumerator2"))))
      (:then_1
        (Timeline|CheckReload PlayFromStart
          (:Finished
            (if (Variables|Default|GetReloadHeld)
              (CallFunction|ChangeAmmo))))))))

(event EventLoadAmmo
  (params (InitialAmmoLoaded :type Float%20%28single-precision%29))
  (Variables|Default|SetAmmoLoaded (Math|Float|Min(Float) (Math|Conversions|ToFloat(Integer) (Utilities|Struct|BreakWeaponClass (select (Variables|Default|GetSlugsLoaded) (Variables|Default|GetSlugs) (Variables|Default|GetWeaponData)))) (Variables|Default|GetAmmoCarried)))
  (Variables|Default|SetAmmoCarried (- (Variables|Default|GetAmmoCarried) (- (Variables|Default|GetAmmoLoaded) InitialAmmoLoaded))))

(fn ConstructionScript
  (|CallParentFunction)
  (Variables|Default|SetAmmoStashed (Math|Conversions|ToFloat(Integer) (Utilities|Struct|BreakWeaponClass (Variables|Default|GetSlugs)))))