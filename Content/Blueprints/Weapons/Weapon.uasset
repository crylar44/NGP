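; Hitscan weapon actor carried by a GLOOM character, firing from the holder's camera and damaging enemy characters and non-spawner structures.
; Construction loads stats from a data table row by WeaponName.
; A state enum and delays drive equipping, holstering, item use and a self-repeating fire loop while the trigger is held.
; Shots apply random cone spread and spawn trail and impact effects; Tick refills auto-recharge ammo after a delay, while reload input only sets a flag.
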(event Custom|ReloadPressed
  (Variables|Default|SetReloadHeld true))

(event Custom|FireAttack
  (params (Damage :type Float%20%28single-precision%29) (Spread :type Float%20%28single-precision%29))
  (bind _returnvalue (Math|Random|RandomFloatinRange 0.0 Spread))
  (bind _returnvalue_2 (Math|Random|RandomFloatinRange 0.0 3.6e+02))
  (bind _holder (Variables|Default|GetHolder))
  (bind _muzzlepointvector (Variables|Default|GetMuzzlePointVector))
  (bind _holder_2 (Variables|Default|GetHolder))
  (bind _weapondata (Variables|Default|GetWeaponData))
  (bind _holder_3 (Variables|Default|GetHolder))
  (bind (_autorechargeammo _rechargedelay) (Utilities|Struct|BreakWeaponClass _weapondata))
  (bind _camera (Variables|/Game/Blueprints/Characters/GLOOM_Character.GLOOM_Character_C|GetCamera _holder))
  (bind _camera_2 (Variables|/Game/Blueprints/Characters/GLOOM_Character.GLOOM_Character_C|GetCamera _holder_2))
  (bind _camera_3 (Variables|/Game/Blueprints/Characters/GLOOM_Character.GLOOM_Character_C|GetCamera _holder_3))
  (bind _returnvalue_3 (Math|Vector|GetForwardVector _camera_2))
  (bind _returnvalue_4 (Math|Vector|GetRightVector _camera_2))
  (bind _returnvalue_5 (Transformation|GetWorldLocation _camera_3))
  (bind _returnvalue_6 (Math|Vector|RotateVectorAroundAxis _returnvalue_3 _returnvalue _returnvalue_4))
  (bind _returnvalue_7 (Math|Vector|RotateVectorAroundAxis _returnvalue_6 _returnvalue_2 _returnvalue_3))
  (bind _returnvalue_8 (* _returnvalue_7 5e+03))
  (bind _returnvalue_9 (+ _returnvalue_5 _returnvalue_8))
  (Utilities|FlowControl|Sequence
    (:then_0
      (bind (_outhit _returnvalue_10) (Collision|LineTraceForObjects _returnvalue_5 _returnvalue_9 (Utilities|Array|MakeArray "ObjectTypeQuery1" "ObjectTypeQuery2" "ObjectTypeQuery3" "ObjectTypeQuery4") false (Utilities|Array|MakeArray (Variables|Default|GetHolder)) "None"))
      (Utilities|FlowControl|Sequence
        (:then_0
          (if _returnvalue_10
            (Utilities|FlowControl|Sequence
              (:then_0
                (CallFunction|HitObject (.HitActor (Collision|BreakHitResult _outhit)) Damage (- _returnvalue_9 _returnvalue_5)))
              (:then_1
                (Effects|SpawnEmitteratLocation (Variables|Default|GetHitEffect) (.ImpactPoint (Collision|BreakHitResult _outhit)) (Math|Conversions|RotationFromXVector (.ImpactNormal (Collision|BreakHitResult _outhit))))))))
        (:then_1
          (Variables|Default|SetFireTime (Utilities|Time|GetGameTimeinSeconds))
          (Game|SpawnActorfromClass (Variables|Default|GetTrailEffect) (Math|Transform|MakeTransform (+ (Transformation|GetWorldLocation _camera) (* (Math|Vector|GetForwardVector _camera) (.x _muzzlepointvector)) (* (Math|Vector|GetRightVector _camera) (.y _muzzlepointvector)) (* (Math|Vector|GetUpVector _camera) (.z _muzzlepointvector))) "0, 0, 0" "1,1,1") "Undefined" 0 (select _returnvalue_10 (.ImpactPoint (Collision|BreakHitResult _outhit)) _returnvalue_9) 0))))
    (:then_1
      (if _autorechargeammo
        (CallFunction|DelayRecharging _rechargedelay)))))

(event Custom|KeepFiring
  (bind _weapondata (Variables|Default|GetWeaponData))
  (bind (_damage _spread) (Utilities|Struct|BreakWeaponClass _weapondata))
  (if (or (> (Variables|Default|GetAmmoLoaded) 0.0) (Variables|Default|GetIgnoreAmmo))
    (Variables|Default|SetAmmoLoaded (Math|Float|Max(Float) (- (Variables|Default|GetAmmoLoaded) 1.0) 0.0))
    (Utilities|FlowControl|Sequence
      (:then_0
        (Variables|Default|SetWeaponState "NewEnumerator4")
        (CallFunction|FireAttack _damage _spread))
      (:then_1
        (Utilities|FlowControl|Delay (/ 1.0 (Utilities|Struct|BreakWeaponClass (Variables|Default|GetWeaponData))))
        (if (Variables|Default|GetTriggerHeld)
          (CallFunction|KeepFiring)
          (else
            (Variables|Default|SetWeaponState "NewEnumerator2")))))
    (else
      (Variables|Default|SetWeaponState "NewEnumerator2"))))

(event Custom|PutAway
  (if (Utilities|Enum|Equal(Enum) (Variables|Default|GetWeaponState) "NewEnumerator2")
    (Variables|Default|SetWeaponState "NewEnumerator1")
    (Utilities|FlowControl|Delay (.PutAwayTime (Utilities|Struct|BreakWeaponClass (Variables|Default|GetWeaponData))))
    (Variables|Default|SetWeaponState "NewEnumerator6")
    (Default|EquipWeapon (Variables|Default|GetHolder))))

(event Custom|TriggerReleased
  (Variables|Default|SetTriggerHeld false))

(event Custom|ReloadReleased
  (Variables|Default|SetReloadHeld false))

(event Custom|TriggerPressed
  (Variables|Default|SetTriggerHeld true)
  (if (Utilities|Enum|Equal(Enum) (Variables|Default|GetWeaponState) "NewEnumerator2")
    (CallFunction|KeepFiring)))

(event Custom|PutUp
  (Variables|Default|SetWeaponState "NewEnumerator0")
  (Utilities|FlowControl|Delay (.PutUpTime (Utilities|Struct|BreakWeaponClass (Variables|Default|GetWeaponData))))
  (if (Variables|Default|GetTriggerHeld)
    (Variables|Default|SetWeaponState "NewEnumerator4")
    (CallFunction|KeepFiring)
    (else
      (Variables|Default|SetWeaponState "NewEnumerator2"))))

(event Custom|PutOffToTheSide
  (params (Duration :type Float%20%28single-precision%29))
  (bind _weapondata (Variables|Default|GetWeaponData))
  (bind (_refill _putofftime _grabagaintime) (Utilities|Struct|BreakWeaponClass _weapondata))
  (Variables|Default|SetWeaponState "NewEnumerator7")
  (Utilities|FlowControl|Delay _putofftime)
  (Variables|Default|SetWeaponState "NewEnumerator8")
  (Utilities|FlowControl|Delay Duration)
  (Variables|Default|SetWeaponState "NewEnumerator9")
  (Utilities|FlowControl|Delay _grabagaintime)
  (if (Variables|Default|GetTriggerHeld)
    (Variables|Default|SetWeaponState "NewEnumerator4")
    (CallFunction|KeepFiring)
    (else
      (Variables|Default|SetWeaponState "NewEnumerator2"))))

(event EventTick
  (params (DeltaSeconds :type Float%20%28single-precision%29))
  (CallFunction|TickRecharge))

(event EventBeginPlay
  (bind _holder (Variables|Default|GetHolder))
  (if (== (Utilities|Array|Get(acopy) (Variables|/Game/Blueprints/Characters/GLOOM_Character.GLOOM_Character_C|GetCarriedWeapons _holder) (Variables|/Game/Blueprints/Characters/GLOOM_Character.GLOOM_Character_C|GetSelectedWeapon _holder)) self)
    (CallFunction|PutUp)))

(fn ConstructionScript
  (bind _returnvalue (Utilities|GetDataTableRow "/Game/System/DataTables/WeaponTable.WeaponTable" (Variables|Default|GetWeaponName))
    (:then
      (bind _output_get (Variables|Default|SetWeaponData _returnvalue))
      (Variables|Default|SetAmmoLoaded (Math|Conversions|ToFloat(Integer) (.AmmoLoad (Utilities|Struct|BreakWeaponClass _output_get))))
      (Variables|Default|SetAmmoCarried (Math|Conversions|ToFloat(Integer) (.AmmoCarrie (Utilities|Struct|BreakWeaponClass _output_get))))
      (Actor|Tick|SetActorTickEnabled (.AutoRechargeAmmo (Utilities|Struct|BreakWeaponClass _output_get)))
      (Variables|Default|SetIgnoreAmmo (== (.AmmoLoad (Utilities|Struct|BreakWeaponClass _output_get)) 0)))))

(fn TraceforPlantingGrenade
  (bind _holder (Variables|Default|GetHolder))
  (bind _camera (Variables|/Game/Blueprints/Characters/GLOOM_Character.GLOOM_Character_C|GetCamera _holder))
  (bind _returnvalue (Transformation|GetWorldLocation _camera))
  (bind (_outhit _returnvalue_2) (Collision|LineTraceForObjects _returnvalue (+ _returnvalue (* (Math|Vector|GetForwardVector _camera) 1e+02)) (Utilities|Array|MakeArray "ObjectTypeQuery1" "ObjectTypeQuery2") false 0 "ForOneFrame"))
  (bind _output_get (Variables|Default|SetReadyToPlant _returnvalue_2))
  (if _output_get
    (Variables|Default|SetPlantLocation (.ImpactPoint (Collision|BreakHitResult _outhit)))
    (Variables|Default|SetPlantNormal (.ImpactNormal (Collision|BreakHitResult _outhit)))))

(fn MuzzlePoint
  (bind _holder (Variables|Default|GetHolder))
  (bind _camera (Variables|/Game/Blueprints/Characters/GLOOM_Character.GLOOM_Character_C|GetCamera _holder))
  (return (+ (Transformation|GetWorldLocation _camera) (Math|Transform|TransformDirection (Math|Transform|MakeTransform "0, 0, 0" (Math|Conversions|RotationFromXVector (Math|Vector|GetForwardVector _camera)) "1,1,1") (Variables|Default|GetMuzzlePointVector)))))

(fn TickRecharge
  (if (and (>= (Utilities|Time|GetGameTimeinSeconds) (Variables|Default|GetRechargeStartTime)) (.AutoRechargeAmmo (Utilities|Struct|BreakWeaponClass (Variables|Default|GetWeaponData))))
    (Variables|Default|SetAmmoLoaded (Math|Float|Min(Float) (Math|Conversions|ToFloat(Integer) (.AmmoLoad (Utilities|Struct|BreakWeaponClass (Variables|Default|GetWeaponData)))) (+ (Variables|Default|GetAmmoLoaded) (* (Utilities|Time|GetWorldDeltaSeconds) 1e+01))))))

(fn DelayRecharging
  (params (Delay :type Float%20%28single-precision%29))
  (Variables|Default|SetRechargeStartTime (Math|Float|Max(Float) (Variables|Default|GetRechargeStartTime) (+ Delay (Utilities|Time|GetGameTimeinSeconds)))))

(fn AimVectorwithSpread
  (params (Spread :type Float%20%28single-precision%29))
  (bind _holder (Variables|Default|GetHolder))
  (bind _camera (Variables|/Game/Blueprints/Characters/GLOOM_Character.GLOOM_Character_C|GetCamera _holder))
  (bind _returnvalue (Math|Vector|GetForwardVector _camera))
  (return (Math|Vector|RotateVectorAroundAxis (Math|Vector|RotateVectorAroundAxis _returnvalue (Math|Random|RandomFloatinRange 0.0 Spread) (Math|Vector|GetRightVector _camera)) (Math|Random|RandomFloatinRange 0.0 3.6e+02) _returnvalue)))

(fn HitObject
  (params (Object :type Object%20Object%20Reference) (Damage :type Float%20%28single-precision%29) (Vector :type Vector))
  (bind _asgloom_character (Utilities|Casting|CastToGLOOM_Character Object)
    (:then
      (if (or (Utilities|Enum|NotEqual(Enum) (Utilities|Struct|BreakClassData (Variables|/Game/Blueprints/Characters/GLOOM_Character.GLOOM_Character_C|GetClassData _asgloom_character)) (Utilities|Struct|BreakClassData (Variables|/Game/Blueprints/Characters/GLOOM_Character.GLOOM_Character_C|GetClassData (Variables|Default|GetHolder)))) (Variables|/Game/Blueprints/Characters/GLOOM_Character.GLOOM_Character_C|GetDead _asgloom_character))
        (Default|TakeDamage _asgloom_character Damage (Math|Vector|Normalize Vector) (Variables|/Game/Blueprints/Characters/GLOOM_Character.GLOOM_Character_C|GetGloomController (Variables|Default|GetHolder)) "NewEnumerator4")))
    (:CastFailed
      (bind _asgloom_structure (Utilities|Casting|CastToGLOOM_Structure Object))
      (if (and (Utilities|Enum|NotEqual(Enum) (.Team (Utilities|Struct|BreakStructureData (Variables|/Game/Blueprints/Structures/GLOOM_Structure.GLOOM_Structure_C|GetStructureData _asgloom_structure))) (Utilities|Struct|BreakClassData (Variables|/Game/Blueprints/Characters/GLOOM_Character.GLOOM_Character_C|GetClassData (Variables|Default|GetHolder)))) (not (.Spawner (Utilities|Struct|BreakStructureData (Variables|/Game/Blueprints/Structures/GLOOM_Structure.GLOOM_Structure_C|GetStructureData _asgloom_structure)))))
        (Default|TakeDamage _asgloom_structure Damage (Variables|/Game/Blueprints/Characters/GLOOM_Character.GLOOM_Character_C|GetGloomController (Variables|Default|GetHolder)))))))

(fn UseItem
  (params (Duration :type Float%20%28single-precision%29))
  (CallFunction|PutOfftotheSide Duration)
  (return (.PutOffTime (Utilities|Struct|BreakWeaponClass (Variables|Default|GetWeaponData)))))