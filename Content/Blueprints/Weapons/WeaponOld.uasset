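; Player-held weapon combining automatic hitscan fire with a secondary trigger for grenades and plantable explosives.
; Tick repeats cooldown-gated shots and charges the secondary, which plants on traced nearby surfaces or otherwise launches a grenade on release.
; Primary press during a charged secondary hold fires a wide shotgun-like burst instead.
; Bullets use random-cone camera traces, spawning trails and impacts and detonating hit Explosives; construction loads WeaponData from a data table.
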(event Custom|PrimeAttackReleased
  (Variables|Default|SetTriggerHeld false))

(event Custom|FireBullet
  (params (Spread :type Float%20%28single-precision%29))
  (bind _returnvalue (Math|Random|RandomFloatinRange 0.0 Spread))
  (bind _returnvalue_2 (Math|Random|RandomFloatinRange 0.0 3.6e+02))
  (bind _holder (Variables|Default|GetHolder))
  (bind _holder_2 (Variables|Default|GetHolder))
  (bind _holder_3 (Variables|Default|GetHolder))
  (bind _camera (Variables|/Game/Blueprints/Characters/GLOOM_Character.GLOOM_Character_C|GetCamera _holder_3))
  (bind _camera_2 (Variables|/Game/Blueprints/Characters/GLOOM_Character.GLOOM_Character_C|GetCamera _holder))
  (bind _camera_3 (Variables|/Game/Blueprints/Characters/GLOOM_Character.GLOOM_Character_C|GetCamera _holder_2))
  (bind _returnvalue_3 (Math|Vector|GetForwardVector _camera_2))
  (bind _returnvalue_4 (Math|Vector|GetRightVector _camera_2))
  (bind _returnvalue_5 (Transformation|GetWorldLocation _camera_3))
  (bind _returnvalue_6 (Math|Vector|RotateVectorAroundAxis _returnvalue_3 _returnvalue _returnvalue_4))
  (bind _returnvalue_7 (Math|Vector|RotateVectorAroundAxis _returnvalue_6 _returnvalue_2 _returnvalue_3))
  (bind _returnvalue_8 (* _returnvalue_7 5e+03))
  (bind _returnvalue_9 (+ _returnvalue_5 _returnvalue_8))
  (bind (_outhit _returnvalue_10) (Collision|LineTraceForObjects _returnvalue_5 _returnvalue_9 (Utilities|Array|MakeArray "ObjectTypeQuery1" "ObjectTypeQuery2" "ObjectTypeQuery7") false 0 "None"))
  (Utilities|FlowControl|Sequence
    (:then_0
      (if _returnvalue_10
        (switch Utilities|FlowControl|Switch|SwitchonECollisionChannel (Collision|GetCollisionObjectType (.HitComponent (Collision|BreakHitResult _outhit)))
          (:ECC_WorldStatic
            (Effects|SpawnEmitteratLocation "/Game/ParticleSystems/BulletImpact.BulletImpact" (.ImpactPoint (Collision|BreakHitResult _outhit)) (Math|Conversions|RotationFromXVector (.ImpactNormal (Collision|BreakHitResult _outhit)))))
          (:ECC_GameTraceChannel1
            (Utilities|Casting|CastToGrenade (.HitActor (Collision|BreakHitResult _outhit))
              (:CastFailed
                (bind _asexplosive (Utilities|Casting|CastToExplosive (.HitActor (Collision|BreakHitResult _outhit))))
                (Default|Explode _asexplosive)))))))
    (:then_1
      (Variables|Default|SetFireTime (Utilities|Time|GetGameTimeinSeconds))
      (Game|SpawnActorfromClass "/Game/Blueprints/Effects/TrailEffect.TrailEffect_C" (Math|Transform|MakeTransform (+ (Transformation|GetWorldLocation _camera) (* (Math|Vector|GetUpVector _camera) -2e+01) (* (Math|Vector|GetRightVector _camera) 15.0)) "0, 0, 0" "1,1,1") "Undefined" 0 (select _returnvalue_10 (.ImpactPoint (Collision|BreakHitResult _outhit)) _returnvalue_9) 0))))

(event Custom|FireGrenade
  (params (TimedGrenade :type Boolean))
  (bind _holder (Variables|Default|GetHolder))
  (bind _camera (Variables|/Game/Blueprints/Characters/GLOOM_Character.GLOOM_Character_C|GetCamera _holder))
  (Game|SpawnActorfromClass "/Game/Blueprints/Projectiles/Grenade.Grenade_C" (Math|Transform|MakeTransform (Transformation|GetWorldLocation _camera) (Math|Conversions|RotationFromXVector (Math|Vector|GetForwardVector _camera)) "1,1,1") "Undefined" 0 0 0))

(event Custom|PlantExplosive
  (Game|SpawnActorfromClass "/Game/Blueprints/Projectiles/Explosive.Explosive_C" (Math|Transform|MakeTransform (Variables|Default|GetPlantLocation) (Math|Conversions|RotationFromXVector (Variables|Default|GetPlantNormal)) "1,1,1") "Undefined" 0 0))

(event Custom|SecondAttackReleased
  (if (Variables|Default|GetGrenadeTriggerHeld)
    (Variables|Default|SetGrenadeTriggerHeld false)
    (if (Variables|Default|GetReadyToPlant)
      (CallFunction|PlantExplosive)
      (else
        (CallFunction|FireGrenade (Variables|Default|GetGrenadeCharged))))))

(event Custom|PrimeAttackPressed
  (if (Variables|Default|GetGrenadeTriggerHeld)
    (if (Variables|Default|GetGrenadeCharged)
      (Variables|Default|SetGrenadeTriggerHeld false)
      (for _index (range 0 24)
        (CallFunction|FireBullet 1e+01)))
    (else
      (Variables|Default|SetTriggerHeld true)
      (if (>= (Utilities|Time|GetGameTimeinSeconds) (+ (Variables|Default|GetFireTime) (Variables|Default|GetCoolDown)))
        (CallFunction|FireBullet 3.0)))))

(event Custom|SecondAttackPressed
  (Variables|Default|SetGrenadeTriggerHeld true)
  (CallFunction|TraceforPlantingGrenade)
  (Variables|Default|SetGrenadeTriggerPressedTime (Utilities|Time|GetGameTimeinSeconds))
  (Variables|Default|SetGrenadeCharged false))

(event EventTick
  (params (DeltaSeconds :type Float%20%28single-precision%29))
  (Utilities|FlowControl|Sequence
    (:then_0
      (if (and (not (Variables|Default|GetGrenadeCharged)) (Variables|Default|GetGrenadeTriggerHeld))
        (if (>= (Utilities|Time|GetGameTimeinSeconds) (+ (Variables|Default|GetGrenadeTriggerPressedTime) (Variables|Default|GetChargeGrenadeTime)))
          (Variables|Default|SetGrenadeCharged true)
          (Development|PrintText "Charged"))))
    (:then_1
      (if (and (Variables|Default|GetTriggerHeld) (>= (Utilities|Time|GetGameTimeinSeconds) (+ (Variables|Default|GetFireTime) (Variables|Default|GetCoolDown))))
        (CallFunction|FireBullet 3.0)
        (elif (Variables|Default|GetGrenadeTriggerHeld)
          (CallFunction|TraceforPlantingGrenade))))))

(fn ConstructionScript
  (bind _returnvalue (Utilities|GetDataTableRow "/Game/System/DataTables/WeaponTable.WeaponTable" (Variables|Default|GetWeaponName))
    (:then
      (Variables|Default|SetWeaponData _returnvalue))))

(fn TraceforPlantingGrenade
  (bind _holder (Variables|Default|GetHolder))
  (bind _camera (Variables|/Game/Blueprints/Characters/GLOOM_Character.GLOOM_Character_C|GetCamera _holder))
  (bind _returnvalue (Transformation|GetWorldLocation _camera))
  (bind (_outhit _returnvalue_2) (Collision|LineTraceForObjects _returnvalue (+ _returnvalue (* (Math|Vector|GetForwardVector _camera) 1e+02)) (Utilities|Array|MakeArray "ObjectTypeQuery1" "ObjectTypeQuery2") false 0 "ForOneFrame"))
  (bind _output_get (Variables|Default|SetReadyToPlant _returnvalue_2))
  (if _output_get
    (Variables|Default|SetPlantLocation (.ImpactPoint (Collision|BreakHitResult _outhit)))
    (Variables|Default|SetPlantNormal (.ImpactNormal (Collision|BreakHitResult _outhit)))))

(fn MuzzlePoint
  (bind _holder (Variables|Default|GetHolder))
  (bind _camera (Variables|/Game/Blueprints/Characters/GLOOM_Character.GLOOM_Character_C|GetCamera _holder))
  (return (+ (Transformation|GetWorldLocation _camera) (Math|Transform|TransformDirection (Math|Transform|MakeTransform "0, 0, 0" (Math|Conversions|RotationFromXVector (Math|Vector|GetForwardVector _camera)) "1,1,1") (Variables|Default|GetMuzzlePointVector)))))