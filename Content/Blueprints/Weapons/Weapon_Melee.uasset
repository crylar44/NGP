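; Melee weapon for GLOOM that strikes along the holder's camera aim, with spread, out to its Reach.
; FireAttack sphere-traces for a target, passes it to HitObject and spawns an impact effect.
; On a miss, a spread-free line trace against static world only places the effect.
; HitObject damages enemy-team characters and structures, sparing spawners unless HurtSpawners is set; an unused copy of this logic remains disconnected.
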(event EventHitObject
  (params (Object :type Object%20Object%20Reference) (Damage :type Float%20%28single-precision%29) (Vector :type Vector :default "0, 0, 0"))
  (bind _asgloom_character (Utilities|Casting|CastToGLOOM_Character Object)
    (:then
      (bind _holderscontroller (Utilities|CheckTeam (.Team (Utilities|Struct|BreakClassData (Variables|/Game/Blueprints/Characters/GLOOM_Character.GLOOM_Character_C|GetClassData _asgloom_character))))
        (:Enemy
          (Default|TakeDamage _asgloom_character Damage Vector _holderscontroller "NewEnumerator4"))))
    (:CastFailed
      (bind _asgloom_structure (Utilities|Casting|CastToGLOOM_Structure Object))
      (bind _holderscontroller_2 (Utilities|CheckTeam (.Team (Utilities|Struct|BreakStructureData (Variables|/Game/Blueprints/Structures/GLOOM_Structure.GLOOM_Structure_C|GetStructureData _asgloom_structure))))
        (:Enemy
          (if (not (.Spawner (Utilities|Struct|BreakStructureData (Variables|/Game/Blueprints/Structures/GLOOM_Structure.GLOOM_Structure_C|GetStructureData _asgloom_structure))))
            (Default|TakeDamage _asgloom_structure Damage _holderscontroller_2)
            (elif (Variables|Default|GetHurtSpawners)
              (Default|TakeDamage _asgloom_structure Damage _holderscontroller_2))))))))

(event EventFireAttack
  (params (Damage :type Float%20%28single-precision%29) (Spread :type Float%20%28single-precision%29))
  (bind _returnvector (CallFunction|AimVectorwithSpread Spread))
  (bind _holder (Variables|Default|GetHolder))
  (bind _holder_2 (Variables|Default|GetHolder))
  (bind _camera (Variables|/Game/Blueprints/Characters/GLOOM_Character.GLOOM_Character_C|GetCamera _holder_2))
  (bind _camera_2 (Variables|/Game/Blueprints/Characters/GLOOM_Character.GLOOM_Character_C|GetCamera _holder))
  (bind _returnvalue (Transformation|GetWorldLocation _camera))
  (bind _returnvalue_2 (Transformation|GetWorldLocation _camera_2))
  (bind (_outhit _returnvalue_3) (Collision|SphereTraceForObjects _returnvalue_2 (+ _returnvalue_2 (* _returnvector (Variables|Default|GetReach))) 0.0 (Utilities|Array|MakeArray "ObjectTypeQuery1" "ObjectTypeQuery3" "ObjectTypeQuery2" "ObjectTypeQuery4") false (Utilities|Array|MakeArray (Variables|Default|GetHolder)) "None"))
  (if _returnvalue_3
    (Utilities|FlowControl|Sequence
      (:then_0
        (CallFunction|HitObject (.HitActor (Collision|BreakHitResult _outhit)) Damage _returnvector))
      (:then_1
        (Effects|SpawnEmitteratLocation "/Game/ParticleSystems/BulletImpact.BulletImpact" (.ImpactPoint (Collision|BreakHitResult _outhit)) (Math|Conversions|RotationFromXVector (.ImpactNormal (Collision|BreakHitResult _outhit))))))
    (else
      (bind (_outhit_2 _returnvalue_4) (Collision|LineTraceForObjects _returnvalue (+ _returnvalue (* (CallFunction|AimVectorwithSpread 0.0) (Variables|Default|GetReach))) (Utilities|Array|MakeArray "ObjectTypeQuery1") false 0 "None"))
      (if _returnvalue_4
        (Effects|SpawnEmitteratLocation "/Game/ParticleSystems/BulletImpact.BulletImpact" (.ImpactPoint (Collision|BreakHitResult _outhit_2)) (Math|Conversions|RotationFromXVector (.ImpactNormal (Collision|BreakHitResult _outhit_2))))))))

(fn ConstructionScript
  (|CallParentFunction))