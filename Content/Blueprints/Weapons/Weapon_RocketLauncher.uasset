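; Rocket launcher weapon Blueprint that fires only while its holder is crouching and ammo is loaded.
; Pulling the trigger switches weapon state and plays the LaunchRocket timeline as a launch delay, which releasing the trigger or standing up cancels.
; If the trigger is still held when the timeline finishes, it consumes one round and spawns a Rocket at the muzzle along the camera's forward vector, crediting the holder's controller as attacker.
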(event EventTriggerPressed
  (Variables|Default|SetTriggerHeld true)
  (if (and (Utilities|Enum|Equal(Enum) (Variables|Default|GetWeaponState) "NewEnumerator2") (Variables|/Game/Blueprints/Characters/GLOOM_Character.GLOOM_Character_C|GetCrouching (Variables|Default|GetHolder)))
    (if (> (Variables|Default|GetAmmoLoaded) 0.0)
      (Variables|Default|SetWeaponState "NewEnumerator4")
      (Timeline|LaunchRocket PlayFromStart
        (:Update
          (if (not (Variables|/Game/Blueprints/Characters/GLOOM_Character.GLOOM_Character_C|GetCrouching (Variables|Default|GetHolder)))
            (Variables|Default|SetTriggerHeld false)
            (if (Utilities|Enum|Equal(Enum) (Variables|Default|GetWeaponState) "NewEnumerator4")
              (Variables|Default|SetWeaponState "NewEnumerator2"))))
        (:Finished
          (if (Variables|Default|GetTriggerHeld)
            (Variables|Default|SetAmmoLoaded (Math|Float|Max(Float) (- (Variables|Default|GetAmmoLoaded) 1.0) 0.0))
            (Game|SpawnActorfromClass "/Game/Blueprints/Projectiles/Rocket.Rocket_C" (Math|Transform|MakeTransform (CallFunction|MuzzlePoint) (Math|Conversions|RotationFromXVector (Math|Vector|GetForwardVector (Variables|/Game/Blueprints/Characters/GLOOM_Character.GLOOM_Character_C|GetCamera (Variables|Default|GetHolder)))) "1,1,1") "Undefined" 0 (Variables|/Game/Blueprints/Characters/GLOOM_Character.GLOOM_Character_C|GetGloomController (Variables|Default|GetHolder)) 0)))))))

(event EventTriggerReleased
  (Variables|Default|SetTriggerHeld false)
  (if (Utilities|Enum|Equal(Enum) (Variables|Default|GetWeaponState) "NewEnumerator4")
    (Variables|Default|SetWeaponState "NewEnumerator2")))

(fn ConstructionScript
  (|CallParentFunction))