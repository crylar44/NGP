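; Shooter weapon Blueprint that extends a parent weapon with timed magazine reloading and camera recoil.
; Reload input checks weapon state and ammo, waits out the reload time, then LoadAmmo refills from carried ammo and resumes firing if the trigger is held.
; FireAttack runs the parent attack, then sends the holder a randomized camera kickback.
; An ammo-consuming fire-rate loop and older ammo math remain as disconnected nodes.
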(event Custom|ReloadPressed
  (Variables|Default|SetReloadHeld true)
  (if (Math|Boolean|ANDBoolean (Utilities|Enum|Equal(Enum) (Variables|Default|GetWeaponState) "NewEnumerator2") (> (Variables|Default|GetAmmoCarried) 0.0) (!= (Variables|Default|GetAmmoLoaded) (Math|Conversions|ToFloat(Integer) (Utilities|Struct|BreakWeaponClass (Variables|Default|GetWeaponData)))))
    (Variables|Default|SetWeaponState "NewEnumerator5")
    (Utilities|FlowControl|Delay (Utilities|Struct|BreakWeaponClass (Variables|Default|GetWeaponData)))
    (CallFunction|LoadAmmo (Variables|Default|GetAmmoLoaded))
    (if (Variables|Default|GetTriggerHeld)
      (CallFunction|KeepFiring)
      (else
        (Variables|Default|SetWeaponState "NewEnumerator2")))))

(event EventFireAttack
  (params (Damage :type Float%20%28single-precision%29) (Spread :type Float%20%28single-precision%29))
  (|CallParentFunction Damage Spread)
  (Default|WeaponKickBack (Variables|Default|GetHolder) (Math|Transform|MakeTransform "-5.000000, 0, 0" (Math|Conversions|RotationFromXVector (Math|Vector|RotateVectorAroundAxis "1.000000, 0, 0" (Math|Random|RandomFloatinRange 3.0 5.0) "0.000000,-1.000000, 0")) "1,1,1")))

(fn ConstructionScript
  (|CallParentFunction))

(fn LoadAmmo
  (params (InitialAmmoLoaded :type Float%20%28single-precision%29))
  (Variables|Default|SetAmmoLoaded (Math|Float|Min(Float) (Math|Conversions|ToFloat(Integer) (Utilities|Struct|BreakWeaponClass (Variables|Default|GetWeaponData))) (Variables|Default|GetAmmoCarried)))
  (Variables|Default|SetAmmoCarried (- (Variables|Default|GetAmmoCarried) (- (Variables|Default|GetAmmoLoaded) InitialAmmoLoaded))))