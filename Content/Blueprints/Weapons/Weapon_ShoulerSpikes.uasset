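; Shoulder spikes weapon that fires a pair of Spike actors from either side of the holder's camera.
; On trigger press, if the weapon state allows and at least two ammo are loaded, it spends two and blocks refiring for a delay set by fire rate.
; Each spike spawns at a camera-relative offset, faces camera forward, carries half the weapon's damage and ignores the holder.
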(event Custom|FireSpike
  (params (OffsetVector :type Vector))
  (bind (_x _y _z) (Math|Vector|BreakVector OffsetVector))
  (bind _holder (Variables|Default|GetHolder))
  (bind _holder_2 (Variables|Default|GetHolder))
  (bind _camera (Variables|/Game/Blueprints/Characters/GLOOM_Character.GLOOM_Character_C|GetCamera _holder))
  (bind _returnvalue (Math|Vector|GetForwardVector _camera))
  (Game|SpawnActorfromClass "/Game/Blueprints/Projectiles/Spike.Spike_C" (Math|Transform|MakeTransform (+ (Transformation|GetWorldLocation _camera) (* _returnvalue _x) (* (Math|Vector|GetRightVector _camera) _y) (* (Math|Vector|GetUpVector _camera) _z)) (Math|Conversions|RotationFromXVector _returnvalue) "1,1,1") "Undefined" 0 (* (Utilities|Struct|BreakWeaponClass (Variables|Default|GetWeaponData)) 0.5) (Variables|/Game/Blueprints/Characters/GLOOM_Character.GLOOM_Character_C|GetGloomController _holder_2) (Utilities|Array|MakeArray _holder_2) 0))

(event EventTriggerPressed
  (if (Utilities|Enum|Equal(Enum) (Variables|Default|GetWeaponState) "NewEnumerator2")
    (if (>= (Variables|Default|GetAmmoLoaded) 2.0)
      (Variables|Default|SetAmmoLoaded (- (Variables|Default|GetAmmoLoaded) 2.0))
      (CallFunction|FireSpike "30.000000,30.000000,20.000000")
      (CallFunction|FireSpike "30.000000,-30.000000,20.000000")
      (Variables|Default|SetWeaponState "NewEnumerator4")
      (Utilities|FlowControl|Delay (/ 1.0 (Utilities|Struct|BreakWeaponClass (Variables|Default|GetWeaponData))))
      (Variables|Default|SetWeaponState "NewEnumerator2"))))

(fn ConstructionScript
  (|CallParentFunction))