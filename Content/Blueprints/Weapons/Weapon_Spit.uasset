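; Spit weapon Blueprint that fires a Spit projectile as its attack.
; On FireAttack it spawns the Spit actor at the muzzle point, aimed along the spread-adjusted aim vector, passing the holder's Gloom controller as attacker plus the damage.
; It then delays recharging by the weapon data's recharge delay.
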(event EventFireAttack
  (params (Damage :type Float%20%28single-precision%29) (Spread :type Float%20%28single-precision%29))
  (Game|SpawnActorfromClass (Variables|Default|GetSpit) (Math|Transform|MakeTransform (CallFunction|MuzzlePoint) (Math|Conversions|RotationFromXVector (CallFunction|AimVectorwithSpread Spread)) "1,1,1") "Undefined" 0 (Variables|/Game/Blueprints/Characters/GLOOM_Character.GLOOM_Character_C|GetGloomController (Variables|Default|GetHolder)) Damage 0)
  (CallFunction|DelayRecharging (Utilities|Struct|BreakWeaponClass (Variables|Default|GetWeaponData))))

(fn ConstructionScript
  (|CallParentFunction))